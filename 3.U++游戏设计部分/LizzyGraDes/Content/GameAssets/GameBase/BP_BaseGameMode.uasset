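; Base game mode that defines shared hooks for running and ending a game, purchase state and battle timing.
; Try-prefixed events forward to run, end and target-actor-rule events, which are empty here apart from EndGame's debug print.
; Setting the purchase condition fires a change dispatcher, and interface functions expose that condition, the game mode and a default cannot-buy answer.
; A helper splits game time into minutes and seconds, while character and pawn accessors remain stubs.
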(event Custom|SetPurchaseConditionWithDelegate
  (params (PurchaseCondition :type Boolean))
  (Variables|Default|SetPurchaseCondition PurchaseCondition)
  (Default|CallOnPurchaseConditionChange))

(event Custom|EndGame
  ;[1 1 1] RunGame and EndGame
  (Development|PrintText "游戏结束。打印来自BaseGameMode的EndGame函数" true true "(R=0.727963,G=0.000000,B=1.000000,A=1.000000)" 1e+01))

(event Custom|RunGame
  ;[1 1 1] RunGame and EndGame
)

(event Custom|GetRulesToSetTargetActor
  (params (ControlledPawn :type BP%20Base%20Character%20Object%20Reference)))

(event Custom|TryToEndGame_1
  ;[1 1 1] RunGame and EndGame
  (CallFunction|EndGame))

(event EventBeginPlay)

(event EventTrytoGetRulestoSetTargetActor
  (params (ControlledPawn :type BP%20Base%20Character%20Object%20Reference))
  (CallFunction|GetRulestoSetTargetActor ControlledPawn))

(event EventTrytoRunGame
  ;[1 1 1] RunGame and EndGame
  (CallFunction|RunGame))

(fn ConstructionScript)

(fn GetBattleTime
  (bind _returnvalue (Utilities|Time|GetGameTimeinSeconds))
  (return _returnvalue (Math|Float|Truncate (/ _returnvalue 6e+01)) (Math|Float|Truncate (Math|Float|%(Float) _returnvalue 6e+01))))

(fn GetPurchaseCondition
  (return (Variables|Default|GetPurchaseCondition)))

(fn BPIGetBaseGameMode
  (return self))

(fn BPIGetCanBuy
  (return false))

(fn BPIGetPurchaseCondition
  (return (Variables|Default|GetPurchaseCondition)))

(fn TrytoGetBaseCharacter
  (return 0))

(fn TrytoGetPlayer0Pawn
  (return 0))

(fn TrytoSetPlayer0Pawn
  (params (ControlledPawn :type BP%20Base%20Character%20Class%20Reference))
  (return 0))