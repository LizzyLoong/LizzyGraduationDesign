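; BP_BaseGameState is a base GameState that provides default responses to game-mode, purchase and turn-based round queries.
; The getters are stubs that return empty, false, zero or first-enum values, presumably for child states to override.
; Its only active logic is two events, named for calls from a turn-based game state, that relay enemy spawn and death through OnEnemySpawned and OnEnemyDeath calls.
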(event EventBeginPlay)

(event EventTick
  (params (DeltaSeconds :type Float%20%28single-precision%29)))

(event EventTrytoCallonEnemySpawnedfromTurnBasedGS
  (Default|CallOnEnemySpawned))

(event EventTrytoCallonEnemyDeathfromTurnBAsedGS
  (Default|CallOnEnemyDeath))

(fn ConstructionScript)

(fn BPIGetBaseGameMode
  (return 0))

(fn BPIGetCanBuy
  (return false))

(fn BPIGetPurchaseCondition
  (return false))

(fn TrytoGetCurrentRoundfromTurnBasedGM
  (return 0))

(fn TrytoGetCurrentRoundPhasefromTurnBasedGM
  (return "NewEnumerator0"))

(fn TrytoGetMaxRoundfromTurnBasedGM
  (return 0))