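; BP_BaseAttackTower is a base Blueprint for attack towers, providing the hooks through which a tower attacks.
; Three TrytoAttack events forward their target actor straight to the matching Attack, Attack2 or Attack3 event, with no checks.
; The Attack events are empty here, leaving the attack behavior to be defined elsewhere, presumably in child towers.
; BeginPlay, Tick and overlap events are disabled placeholders, and the construction script only calls its parent.
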(event Custom|Attack3
  (params (TargetActor :type BP%20Base%20Character%20Object%20Reference)))

(event Custom|Attack2
  (params (TargetActor :type BP%20Base%20Character%20Object%20Reference)))

(event EventBeginPlay
  (|CallParentFunction) ; 此节点被禁用，将不会被调用。\n从引脚连出引线来编译功能。
)

(event Collision|EventActorBeginOverlap
  (params (OtherActor :type Actor%20Object%20Reference))
  (|CallParentFunction OtherActor) ; 此节点被禁用，将不会被调用。\n从引脚连出引线来编译功能。
)

(event EventTick
  (params (DeltaSeconds :type Float%20%28single-precision%29))
  (|CallParentFunction DeltaSeconds) ; 此节点被禁用，将不会被调用。\n从引脚连出引线来编译功能。
)

(event EventAttack
  (params (TargetActor :type BP%20Base%20Character%20Object%20Reference)))

(event EventTrytoAttack
  (params (TargetActor :type BP%20Base%20Character%20Object%20Reference))
  (CallFunction|Attack TargetActor))

(event EventTrytoAttack2
  (params (TargetActor :type BP%20Base%20Character%20Object%20Reference))
  (CallFunction|Attack2 TargetActor))

(event EventTrytoAttack3
  (params (TargetActor :type BP%20Base%20Character%20Object%20Reference))
  (CallFunction|Attack3 TargetActor))

(fn ConstructionScript
  (|CallParentFunction))