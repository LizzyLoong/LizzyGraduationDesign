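; BP_BaseConstruction is a base pawn for constructions, built with a character movement component, an ability system and an HP bar widget.
; On BeginPlay it disables movement so the construction stays in place, then binds a handler to its HP change event.
; The handler divides the new HP by an ability system attribute and sends the ratio to the bar through an interface call.
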(event Custom|HPChangeEvent_事件_1
  (params (OldValue :type Float%20%28single-precision%29) (NewValue :type Float%20%28single-precision%29))
  (Class|BPIWBPStateBar|BPIUpdateHP(Message) (UserInterface|GetUserWidgetObject (Variables|Default|GetHPBar)) (/ NewValue (.ReturnValue (Ability|Attribute|GetFloatAttributefromAbilitySystemComponent (Variables|Default|GetAbilitySystem) "(AttributeName=\"MaxHP\",Attribute=/Script/LizzyGraDes.CPP_BaseAttributeSet:MaxHP,AttributeOwner=\"/Script/CoreUObject.Class'/Script/LizzyGraDes.CPP_BaseAttributeSet'\")")))))

(event EventBeginPlay
  (Utilities|FlowControl|Sequence
    (:then_0
      (Pawn|Components|CharacterMovement|DisableMovement (Variables|Character|GetCharacterMovement)))
    (:then_1
      (EventDispatchers|AssignHPChangeEvent (delegate Custom|HPChangeEvent_事件_1)))))

(event Collision|EventActorBeginOverlap
  (params (OtherActor :type Actor%20Object%20Reference)))

(event EventTick
  (params (DeltaSeconds :type Float%20%28single-precision%29)))

(fn ConstructionScript)