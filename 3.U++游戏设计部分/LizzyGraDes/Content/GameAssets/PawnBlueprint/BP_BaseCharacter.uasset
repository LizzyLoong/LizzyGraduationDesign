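; Base character Blueprint built on GAS, providing shared stats, combat hooks and death handling for BP_Legends and other characters.
; Attribute change events drive walk speed, capsule scale, floating damage numbers and death, which plays sound and montage, then notifies GameState and destroys non-Legends actors.
; Attack and six skill slots forward targets to dispatchers, leaving logic to subclasses.
; Also provides move/rotate input, cursor-hover highlight, impulse dash and launch helpers, and target accessors.
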(event OnBeginCursorOver(Mesh)
  (params (TouchedComponent :type Primitive%20Component%20Object%20Reference))
  ;[1 1 1] 鼠标选中红框
  (Rendering|Material|SetOverlayMaterial (Variables|Character|GetMesh) "/Game/GameAssets/PawnBlueprint/UI/Cursor/Highlight/MI_EnemyHighlight.MI_EnemyHighlight" :!class /Script/Engine.MeshComponent))

(event OnEndCursorOver(Mesh)
  (params (TouchedComponent :type Primitive%20Component%20Object%20Reference))
  ;[1 1 1] 鼠标选中红框
  (Rendering|Material|SetOverlayMaterial (Variables|Character|GetMesh) 0 :!class /Script/Engine.MeshComponent))

(event Custom|HPChangeEvent_事件_0
  (params (OldValue :type Float%20%28single-precision%29) (NewValue :type Float%20%28single-precision%29))
  (if (<= NewValue 1.0)
    (CallFunction|KillCharacter (Variables|Character基础|GetDying%20Sound) (Variables|Character基础|GetDying%20Anim))))

(event Custom|KillCharacter
  (params (Dying%20Sound :type Sound%20Base%20Object%20Reference) (Dying%20Anim :type Anim%20Montage%20Object%20Reference))
  ;[1 1 1] 处理角色死亡
  (Audio|PlaySoundatLocation Dying%20Sound (Transformation|GetActorLocation) "0, 0, 0" 1.0 1.0 0.0 0 0 0 0)
  (bind _returnvalue (Animation|PlayAnimMontage Dying%20Anim 1.0 "None"))
  (Utilities|Time|SetTimerbyEvent (delegate Custom|处理死亡事件) (Math|Float|Max(Float) _returnvalue 0.1)))

(event Custom|处理死亡事件
  ;[1 1 1] 处理角色死亡
  (Default|CallOnCharacterDeath)
  (if (Utilities|ClassIsChildOf (Utilities|GetClass self) "/Game/GameAssets/PawnBlueprint/Legends/BP_Legends.BP_Legends_C")
    _
    (else
      (Actor|DestroyActor)))
  (Class|BPITurnBased|TrytoCallonEnemyDeathfromTurnBAsedGS(Message) (Game|GetGameState)))

(event EventBeginPlay
  (|CallParentFunction)
  (Utilities|FlowControl|Sequence
    (:then_0
      (bind _asbp_base_player_controller (Utilities|Casting|CastToBP_BasePlayerController (Game|GetPlayerController 0)))
      (Variables|Default|SetAs%20BP%20Player%20Controller _asbp_base_player_controller)
      (Variables|Default|SetActor半高 (.z (Transformation|GetWorldLocation (Variables|Default|GetFootTransform)))))
    (:then_1
      (|WalkSpeedUpdate)
      (|ScaleUpdate))
    (:then_2
      (Class|AbilitySystemComponent|GiveAbilityandActivateOnce (Variables|Default|GetAbilitySystem) "/Game/GameAssets/PawnBlueprint/GA_BaseRecover.GA_BaseRecover_C" 0 -1))
    (:then_3
      (|伤害飘字))))

(event Collision|EventActorBeginOverlap
  (params (OtherActor :type Actor%20Object%20Reference)))

(event Custom|UsingSkill5
  (params (TargetActor :type BP%20Base%20Character%20Object%20Reference))
  ;[1 1 1] Skill5
  (Default|CallOnSkill5Activate TargetActor))

(event Custom|UsingSkill1
  (params (TargetActor :type BP%20Base%20Character%20Object%20Reference))
  ;[1 1 1] Skill1
  (Default|CallOnSkill1Activate TargetActor))

(event Custom|UsingSkill2
  (params (TargetActor :type BP%20Base%20Character%20Object%20Reference))
  ;[1 1 1] Skill2
  (Default|CallOnSkill2Activate TargetActor))

(event Custom|Attack
  (params (TargetActor :type BP%20Base%20Character%20Object%20Reference))
  ;[1 1 1] 默认攻击逻辑，需要在子类中实现的是Attack的逻辑
  (Default|CallOnAttackActivate TargetActor))

(event Custom|UsingSkill3
  (params (TargetActor :type BP%20Base%20Character%20Object%20Reference))
  ;[1 1 1] Skill3
  (Default|CallOnSkill3Activate TargetActor))

(event Custom|UsingSkill0
  (params (Target :type BP%20Base%20Character%20Object%20Reference))
  ;[1 1 1] Skill0
  (Default|CallOnSkill0Activate Target))

(event Custom|UsingSkill4
  (params (TargetActor :type BP%20Base%20Character%20Object%20Reference))
  ;[1 1 1] Skill4
  (Default|CallOnSkill4Activate TargetActor))

(event Input|EnhancedActionEvents|EnhancedInputActionCC_Move
  (params (ActionValue :type Vector%202D%20Structure) (ElapsedSeconds :type Float%20%28double-precision%29) (TriggeredSeconds :type Float%20%28double-precision%29) (InputAction :type Input%20Action%20Object%20Reference :default "/Game/GameAssets/Input/CC/CC_Move.CC_Move"))
  (Pawn|Input|AddMovementInput (Math|Vector|MakeVector (.x ActionValue) (.y ActionValue) 0.0) 1.0 false))

(event Input|EnhancedActionEvents|EnhancedInputActionCC_Rotate
  (params (ActionValue :type Vector%202D%20Structure) (ElapsedSeconds :type Float%20%28double-precision%29) (TriggeredSeconds :type Float%20%28double-precision%29) (InputAction :type Input%20Action%20Object%20Reference :default "/Game/GameAssets/Input/CC/CC_Rotate.CC_Rotate"))
  (CallFunction|设置角色朝向 self (Math|Vector|MakeVector (.x ActionValue) (.y ActionValue) 0.0))
  (Development|PrintText "Hello"))

(event EventTrytoCallSkill4
  (params (TargetActor :type BP%20Base%20Character%20Object%20Reference))
  ;[1 1 1] Skill4
  (Utilities|IsValid TargetActor
    (:Is%20Valid
      (CallFunction|UsingSkill4 TargetActor))
    (:Is%20Not%20Valid
      (CallFunction|UsingSkill4 (Variables|Default|GetTargetActor)))))

(event EventTrytoCallSkill3
  (params (TargetActor :type BP%20Base%20Character%20Object%20Reference))
  ;[1 1 1] Skill3
  (Utilities|IsValid TargetActor
    (:Is%20Valid
      (CallFunction|UsingSkill3 TargetActor))
    (:Is%20Not%20Valid
      (CallFunction|UsingSkill3 (Variables|Default|GetTargetActor)))))

(event EventTrytoCallSkill2
  (params (TargetActor :type BP%20Base%20Character%20Object%20Reference))
  ;[1 1 1] Skill2
  (Utilities|IsValid TargetActor
    (:Is%20Valid
      (CallFunction|UsingSkill2 TargetActor))
    (:Is%20Not%20Valid
      (CallFunction|UsingSkill2 (Variables|Default|GetTargetActor)))))

(event EventTrytoCallSkill1
  (params (TargetActor :type BP%20Base%20Character%20Object%20Reference))
  ;[1 1 1] Skill1
  (Utilities|IsValid TargetActor
    (:Is%20Valid
      (CallFunction|UsingSkill1 TargetActor))
    (:Is%20Not%20Valid
      (CallFunction|UsingSkill1 (Variables|Default|GetTargetActor)))))

(event EventTrytoCallSkill0
  (params (TargetActor :type BP%20Base%20Character%20Object%20Reference))
  ;[1 1 1] Skill0
  (Utilities|IsValid TargetActor
    (:Is%20Valid
      (CallFunction|UsingSkill0 TargetActor))
    (:Is%20Not%20Valid
      (CallFunction|UsingSkill0 (Variables|Default|GetTargetActor)))))

(event EventTrytoAttack
  (params (TargetActor :type BP%20Base%20Character%20Object%20Reference))
  ;[1 1 1] 默认攻击逻辑，需要在子类中实现的是Attack的逻辑
  (Utilities|IsValid TargetActor
    (:Is%20Valid
      (CallFunction|Attack TargetActor))
    (:Is%20Not%20Valid
      (CallFunction|Attack (Variables|Default|GetTargetActor)))))

(event EventTrytoCallSkill5
  (params (TargetActor :type BP%20Base%20Character%20Object%20Reference))
  ;[1 1 1] Skill5
  (Utilities|IsValid TargetActor
    (:Is%20Valid
      (CallFunction|UsingSkill5 TargetActor))
    (:Is%20Not%20Valid
      (CallFunction|UsingSkill5 (Variables|Default|GetTargetActor)))))

(fn ConstructionScript
  (Variables|/Script/Engine.CharacterMovementComponent|SetMaxWalkSpeed (Variables|Character|GetCharacterMovement) (CallFunction|GetAttributeValue "(AttributeName=\"Run\",Attribute=/Script/LizzyGraDes.CPP_BaseAttributeSet:Run,AttributeOwner=\"/Script/CoreUObject.Class'/Script/LizzyGraDes.CPP_BaseAttributeSet'\")"))
  (Variables|Default|SetActor半高 (.z (Transformation|GetWorldLocation (Variables|Default|GetFootTransform)))))

(fn 获取技能标签组中指定技能
  (params (组中Index :type Integer))
  (return (Utilities|Array|Get(acopy) (Variables|Character基础|Get技能标签组) 组中Index)))

(fn 获取运动方向
  (bind _returnvalue (Transformation|GetVelocity))
  (bind _returnvalue_2 (Class|KismetMathLibrary|VectorNormal2D _returnvalue 0.0001))
  (if (Utilities|Operators|EqualEqual :A _returnvalue_2)
    (return (Transformation|GetActorForwardVector))
    (else
      (return _returnvalue_2))))

(fn GetAttributeValue
  (params (Attribute :type Gameplay%20Attribute%20Structure))
  (return (.ReturnValue (Ability|Attribute|GetFloatAttributefromAbilitySystemComponent (Variables|Default|GetAbilitySystem) Attribute))))

(fn IsActoronGround
  (bind _foottransform (Variables|Default|GetFootTransform))
  (bind _returnvalue (Transformation|GetWorldLocation _foottransform))
  (bind (_outhit _returnvalue_2) (Collision|LineTraceByChannel _returnvalue (- _returnvalue (Math|Vector|MakeVector 0.0 0.0 (+ (Variables|Default|GetActor半高) 1e+01))) "TraceTypeQuery1" false 0 "Persistent"))
  (return _outhit _returnvalue_2))

(fn Dash
  (params (Direction（NeedToNormalize） :type Vector) (Dist :type Float%20%28double-precision%29))
  (Physics|AddImpulse (Variables|Character|GetCharacterMovement) (* Direction（NeedToNormalize） (* Dist 2e+05)) false))

(fn DashAir
  (params (Direction（NeedToNormalize） :type Vector) (Dist（以击飞高度1为单位） :type Float%20%28double-precision%29))
  (Physics|AddImpulse (Variables|Character|GetCharacterMovement) (* Direction（NeedToNormalize） (* Dist（以击飞高度1为单位） 1e+04)) false))

(fn Air
  (params (击飞高度（给值建议1，2） :type Float%20%28double-precision%29))
  (Physics|AddImpulse (Variables|Character|GetCharacterMovement) (* (Transformation|GetActorUpVector) (* 击飞高度（给值建议1，2） 500)) true)
  (return))

(fn BPIGetBaseGameMode
  (return 0))

(fn BPIGetCanBuy
  (return false))

(fn BPIGetPurchaseCondition
  (return false))

(event Custom|RunChangeEvent_事件
  (params (OldValue :type Float%20%28single-precision%29) (NewValue :type Float%20%28single-precision%29))
  (Variables|/Script/Engine.CharacterMovementComponent|SetMaxWalkSpeed (Variables|Character|GetCharacterMovement) NewValue))

(event Custom|自定义事件
  (Variables|Default|SetActor半高 (.z (Transformation|GetWorldLocation (Variables|Default|GetFootTransform)))))

(event Custom|ToughChangeEvent_事件
  (params (OldValue :type Float%20%28single-precision%29) (NewValue :type Float%20%28single-precision%29))
  (Transformation|SetWorldScale3D (Variables|Default|GetCapsuleComponent) (* "1.000000,1.000000,1.000000" (+ (/ NewValue 100) (.x (Transformation|GetActorScale3D)))))
  (Utilities|Time|SetTimerbyEvent (delegate Custom|自定义事件) 0.1))

(event Custom|HPChangeEvent_事件
  (params (OldValue :type Float%20%28single-precision%29) (NewValue :type Float%20%28single-precision%29))
  (bind _returnvalue (- OldValue NewValue))
  (if (and (<= OldValue (CallFunction|GetAttributeValue "(AttributeName=\"MaxHP\",Attribute=/Script/LizzyGraDes.CPP_BaseAttributeSet:MaxHP,AttributeOwner=\"/Script/CoreUObject.Class'/Script/LizzyGraDes.CPP_BaseAttributeSet'\")")) (> _returnvalue 1.0))
    (bind _returnvalue_2 (UserInterface|CreateWidget "/Game/GameAssets/PawnBlueprint/UI/WBP_DamageShow.WBP_DamageShow_C" 0 _returnvalue))
    (Class|UserWidget|SetPositioninViewport _returnvalue_2 (.ScreenPosition (Class|GameplayStatics|ProjectWorldtoScreen (Game|GetPlayerController 0) (Transformation|GetActorLocation self) false)) true)
    (UserInterface|Viewport|AddtoViewport _returnvalue_2 0)
    ;[1 1 1] 死亡逻辑
    (if (<= NewValue 5.0)
      (CallFunction|KillCharacter (Variables|Character基础|GetDying%20Sound) (Variables|Character基础|GetDying%20Anim)))))

(fn TrytoGetBaseCharacter
  (return self))

(fn TrytoGetPlayer0Pawn
  (return 0))

(fn TrytoGetSkill0Collision
  (return 0 0 0))

(fn TrytoGetSkill1Collision
  (return 0 0 0))

(fn TrytoGetSkill2Collision
  (return 0 0 0))

(fn TrytoGetSkill3Collision
  (return 0 0 0))

(fn TrytoGetSkill4Collision
  (return 0 0 0))

(fn TrytoGetSkill5Collision
  (return 0 0 0))

(fn TrytoGetTargetActor
  (return (Variables|Default|GetTargetActor)))

(fn TrytoSetPlayer0Pawn
  (params (ControlledPawn :type BP%20Base%20Character%20Class%20Reference))
  (return 0))

(fn TrytoSetTargetActor
  (params (TargetActer :type BP%20Base%20Character%20Object%20Reference))
  (bind _output_get (Variables|Default|SetTargetActor TargetActer))
  (return _output_get))