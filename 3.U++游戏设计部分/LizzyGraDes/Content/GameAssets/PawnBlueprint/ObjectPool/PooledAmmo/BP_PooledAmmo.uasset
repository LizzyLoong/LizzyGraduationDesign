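; Pooled projectile actor that flies via its AmmoMovement component and returns itself to the pool after LivingTime.
; SetInUse calls the parent, clears the lifetime timer and, on activation, restarts it and launches along the actor's forward vector at the stored Speed.
; When the timer fires, it calls SetInUse(false) instead of destroying the actor.
; TrytoInit events forward to velocity setters that store Speed and use either actor forward or a supplied direction.
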(event Custom|InitVelocityWithTransform
  (params (Speed :type Integer) (ForwardVector :type Vector))
  ;[1 1 1] 初始化速度
  (Variables|/Script/Engine.MovementComponent|SetVelocity (Variables|Default|GetAmmoMovement) (* ForwardVector Speed))
  (Variables|Default|SetSpeed Speed))

(event Custom|InitVelocity
  (params (Speed :type Integer))
  ;[1 1 1] 初始化速度
  (Variables|/Script/Engine.MovementComponent|SetVelocity (Variables|Default|GetAmmoMovement) (* (Transformation|GetActorForwardVector) Speed))
  (Variables|Default|SetSpeed Speed))

(event Custom|将正在使用的放入池中
  (CallFunction|SetinUse false))

(event EventBeginPlay
  (|CallParentFunction))

(event Collision|EventActorBeginOverlap
  (params (OtherActor :type Actor%20Object%20Reference)))

(event EventTick
  (params (DeltaSeconds :type Float%20%28single-precision%29)))

(event EventTrytoInitVelocity
  (params (Speed :type Integer))
  ;[1 1 1] 初始化速度
  (CallFunction|InitVelocity Speed))

(event EventTrytoInitVelocitywithForwardVector
  (params (Speed :type Integer) (ForwardVector :type Vector :default "0, 0, 0"))
  ;[1 1 1] 初始化速度
  (CallFunction|InitVelocitywithTransform Speed ForwardVector))

(event EventSetinUse
  (params (InUse :type Boolean))
  (|CallParentFunction InUse)
  (Utilities|Time|ClearandInvalidateTimerbyHandle (Variables|Default|Get存活时间定时器))
  (if InUse
    (bind _returnvalue (Utilities|Time|SetTimerbyEvent (delegate Custom|将正在使用的放入池中) (Variables|Default|GetLivingTime)))
    (Variables|Default|Set存活时间定时器 _returnvalue)
    (Variables|/Script/Engine.MovementComponent|SetVelocity (Variables|Default|GetAmmoMovement) (* (Transformation|GetActorForwardVector) (Variables|Default|GetSpeed)))))

(fn ConstructionScript
  (|CallParentFunction))