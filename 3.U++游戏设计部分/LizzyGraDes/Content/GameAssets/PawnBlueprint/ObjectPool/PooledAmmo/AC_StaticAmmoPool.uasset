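; Actor component that provides a fixed-size object pool of BP_PooledAmmo projectiles for its owner.
; On BeginPlay it pre-spawns the pool at the owner's transform and marks every ammo actor as not in use.
; SpawnAmmoFronPool linearly searches for free ammo, then moves it, sets speed and living time, and activates it instead of spawning.
; It prints a failure message if the search returns no valid actor.
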(event EventBeginPlay
  (bind _returnvalue (Components|GetOwner))
  (for _index (range 0 (Variables|Default|GetPooledSize))
    (bind _asbp_pooled_ammo (Utilities|Casting|CastToBP_PooledAmmoClass (Variables|Default|GetPooledActorClass)))
    (bind _returnvalue_2 (Game|SpawnActorfromClass _asbp_pooled_ammo (Transformation|GetActorTransform _returnvalue) "Undefined" "MultiplyWithRoot" _returnvalue 50 0.5 0))
    (Default|SetinUse _returnvalue_2 false)
    (Utilities|Array|AddUnique (Variables|AmmoPool配置|GetPooledAmmo) _returnvalue_2)))

(event EventTick
  (params (DeltaSeconds :type Float%20%28single-precision%29))
  (|CallParentFunction DeltaSeconds) ; 此节点被禁用，将不会被调用。\n从引脚连出引线来编译功能。
)

(fn FindFirstAvaliableAmmo
  (bind _array_element (Utilities|Array|ForEachLoopwithBreak (Variables|AmmoPool配置|GetPooledAmmo) :!label _label)
    (:LoopBody
      (if (not (Variables|/Game/GameAssets/PawnBlueprint/ObjectPool/BP_PooledActor.BP_PooledActor_C|GetInUse _array_element))
        (goto _label Break)))
    (:Completed
      (return _array_element))))

(fn SpawnAmmoFronPool
  (params (SpawnTransform :type Transform) (LivingTime :type Float%20%28double-precision%29) (Speed :type Integer))
  (bind _array_element (CallFunction|FindFirstAvaliableAmmo))
  (Utilities|IsValid _array_element
    (:Is%20Valid
      (Transformation|SetActorTransform _array_element SpawnTransform)
      (Variables|/Game/GameAssets/PawnBlueprint/ObjectPool/PooledAmmo/BP_PooledAmmo.BP_PooledAmmo_C|SetSpeed _array_element Speed)
      (Variables|/Game/GameAssets/PawnBlueprint/ObjectPool/PooledAmmo/BP_PooledAmmo.BP_PooledAmmo_C|SetLivingTime _array_element LivingTime)
      (Default|SetinUse _array_element true)
      (return _array_element))
    (:Is%20Not%20Valid
      (Development|PrintText "从池中生成失败"))))