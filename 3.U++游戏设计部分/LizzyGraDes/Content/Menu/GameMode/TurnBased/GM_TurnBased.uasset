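; Game mode for a round-based enemy wave mode that cycles through start, preparation, battle and end phases via a phase-change dispatcher.
; Preparation opens purchasing and runs a timer, then spawns random behavior-tree enemies around the player and closes purchasing.
; Battle counts enemy deaths from GS_TurnBased to advance rounds until the maximum ends the game.
; It also takes the default pawn from the GameInstance and assigns AI targets from BP_Legends.
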(event Custom|OnRoundPhaseChange_Event
  (switch Utilities|FlowControl|Switch|SwitchonE_RoundPhase (Variables|回合制基础|GetCurrentRoundPhase)
    (:NewEnumerator0
      (Mode基础|ChangePhaseOccuredOn开始阶段))
    (:NewEnumerator2
      (|准备阶段行为))
    (:NewEnumerator1
      (|即将结束战斗阶段))
    (:NewEnumerator3
      (Mode基础|ChangePhaseOccuredOn结束阶段))))

(event EventBeginPlay
  (|CallParentFunction)
  (Utilities|FlowControl|Sequence
    (:then_0
      (bind _returnvalue (UserInterface|CreateWidget "/Game/Menu/GameMode/TurnBased/UI/WBP_TurnBased.WBP_TurnBased_C"))
      (bind _output_get (Variables|Default|Set模式UI _returnvalue))
      (UserInterface|Viewport|AddtoViewport _output_get 0))
    (:then_1
      (Mode基础|ChangeTargetRoundPhase "NewEnumerator0")
      (EventDispatchers|BindEventtoOnRoundPhaseChange (delegate Custom|OnRoundPhaseChange_Event)))))

(event EventRunGame
  ;[1 1 1] 默认应该是在开始阶段才能调用该函数，会直接转到准备阶段
  (CallFunction|ChangeRoundPhase true))

(event EventGetRulestoSetTargetActor
  (params (ControlledPawn :type BP%20Base%20Character%20Object%20Reference))
  (bind _outactors (Actor|GetAllActorsOfClass "/Game/GameAssets/PawnBlueprint/Legends/BP_Legends.BP_Legends_C"))
  (Class|BPIBaseCharacter|TrytoSetTargetActor(Message) (Pawn|GetControlledPawn (AI|GetAIController ControlledPawn)) (Utilities|Array|Get(acopy) _outactors)))

(event EventTrytoGetRulestoSetTargetActor
  (params (ControlledPawn :type BP%20Base%20Character%20Object%20Reference))
  (CallFunction|GetRulestoSetTargetActor ControlledPawn))

(fn ConstructionScript
  (|CallParentFunction)
  (bind _player0pawn (Class|BPIBaseGameplayMessage|TrytoGetPlayer0Pawn(Message) (Game|GetGameInstance)))
  (Variables|Default|SetDefaultPawnClass _player0pawn))

(fn ChangeTargetRoundPhase
  (params (RoundPhase :type E_RoundPhase%20Enum :default "NewEnumerator0"))
  (switch Utilities|FlowControl|Switch|SwitchonE_RoundPhase RoundPhase
    (:NewEnumerator0
      (Variables|回合制基础|SetCurrentRoundPhase "NewEnumerator0")
      (Default|CallOnRoundPhaseChange))
    (:NewEnumerator2
      (Variables|回合制基础|SetCurrentRoundPhase "NewEnumerator2")
      (Default|CallOnRoundPhaseChange))
    (:NewEnumerator1
      (Variables|回合制基础|SetCurrentRoundPhase "NewEnumerator1")
      (Default|CallOnRoundPhaseChange))
    (:NewEnumerator3
      (Variables|回合制基础|SetCurrentRoundPhase "NewEnumerator3")
      (Default|CallOnRoundPhaseChange))))

(fn ChangePhaseOccuredOn开始阶段
  (Variables|Default|SetCanChangePhase false)
  (Mode基础|ChangeTargetRoundPhase "NewEnumerator2")
  (CallFunction|SetPurchaseConditionwithDelegate true)
  (Variables|Default|SetCanChangePhase true))

(fn ChangePhaseOccuredOn准备阶段
  (params (PawnClass :type Array%20of%20Pawn%20Class%20References) (生成位置中心 :type Vector%20%28by%20ref%29) (生成范围半径 :type Float%20%28single-precision%29))
  (for _index (range 1 (Variables|Default|GetRoundCount))
    (CallFunction|SpawnEnemyinEachRound (Utilities|Array|Get(acopy) PawnClass (Math|Random|RandomInteger (Utilities|Array|Length PawnClass))) (.RandomLocation (AI|Navigation|GetRandomReachablePointinRadius (Math|Vector|MakeVector (.x 生成位置中心) (.y 生成位置中心) (+ (.z 生成位置中心) 1e+02)) 生成范围半径 0 0))))
  (Mode基础|ChangeTargetRoundPhase "NewEnumerator1")
  (CallFunction|SetPurchaseConditionwithDelegate false))

(fn ChangePhaseOccuredOn战斗阶段
  (if (> (Variables|回合制基础|GetCurrentRound) (Variables|回合制基础|GetMaxRound))
    (Mode基础|ChangeTargetRoundPhase "NewEnumerator3")
    (else
      (Mode基础|ChangeTargetRoundPhase "NewEnumerator2")
      (CallFunction|SetPurchaseConditionwithDelegate true)
      (Math|Integer|IncrementInt (Variables|回合制基础|GetCurrentRound)
        (:%20%20
          (Default|CallOnCurrentRoundChanged))))))

(fn ChangePhaseOccuredOn结束阶段
  (CallFunction|EndGame))

(fn ChangeRoundPhase
  (params (Condition :type Boolean))
  (if Condition
    (Default|CallOnRoundPhaseChange)))

(fn SpawnEnemyinEachRound
  (params (PawnClass :type Pawn%20Class%20Reference) (Location :type Vector))
  (AI|SpawnAIFromClass PawnClass "/Game/GameAssets/PawnBlueprint/AI/BT_BaseTree.BT_BaseTree" Location "0, 0, 0" true 0)
  (Class|BPITurnBased|TrytoCallonEnemySpawnedfromTurnBasedGS(Message) (Game|GetGameState)))

(event Custom|OnEnemyDeath_事件
  (bind _result (Math|Integer|DecrementInt (Variables|Default|GetCurrentCount))
    (:%20%20
      (if (<= _result 0)
        (Mode基础|ChangePhaseOccuredOn战斗阶段)))))

(event Custom|准备阶段结束后
  (Utilities|Time|ClearandInvalidateTimerbyHandle (Variables|Timer|GetTimer))
  (Mode基础|ChangePhaseOccuredOn准备阶段 (Variables|Default|GetEnemyClasses) (Transformation|GetActorLocation (Pawn|GetControlledPawn (Game|GetPlayerController 0))) 1e+03))

(fn TrytoGetCurrentRoundfromTurnBasedGM
  (return 0))

(fn TrytoGetCurrentRoundPhasefromTurnBasedGM
  (return (Variables|回合制基础|GetCurrentRoundPhase)))

(fn TrytoGetMaxRoundfromTurnBasedGM
  (return (Variables|回合制基础|GetMaxRound)))