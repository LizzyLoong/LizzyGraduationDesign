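; Turn-based Defence game mode that makes the base the target for AI-controlled pawns.
; Its target rule event finds all BP_Base actors and sends the first to the pawn, fetched through its AI controller, via a TryToSetTargetActor interface message.
; EndGame and construction only call the parent, and the BeginPlay and Tick events are inactive.
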(event EventBeginPlay
  (|CallParentFunction) ; 此节点被禁用，将不会被调用。\n从引脚连出引线来编译功能。
)

(event EventTick
  (params (DeltaSeconds :type Float%20%28single-precision%29)))

(event EventGetRulestoSetTargetActor
  (params (ControlledPawn :type BP%20Base%20Character%20Object%20Reference))
  (bind _outactors (Actor|GetAllActorsOfClass "/Game/GameAssets/PawnBlueprint/Construction/Base/BP_Base.BP_Base_C"))
  (Class|BPIBaseCharacter|TrytoSetTargetActor(Message) (Pawn|GetControlledPawn (AI|GetAIController ControlledPawn)) (Utilities|Array|Get(acopy) _outactors)))

(event EventEndGame
  (|CallParentFunction))

(fn ConstructionScript
  (|CallParentFunction))