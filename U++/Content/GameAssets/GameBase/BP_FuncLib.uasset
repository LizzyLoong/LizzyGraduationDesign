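; BP_FuncLib is a Blueprint function library of small, independent actor and randomness helpers for gameplay.
; It gets a normalized 2D direction between two actors and rotates an actor to face a given vector.
; It also rolls a percentage chance alongside a 0–100 random number.
; A random-point helper offsets an actor's location within an integer radius, keeping X and Y and setting world Z to zero.
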(fn 获取两Actor之间位置信息
  (params (SourceActor :type Actor%20Object%20Reference) (TargetActor :type Actor%20Object%20Reference))
  (return (Class|KismetMathLibrary|VectorNormal2D (- (Transformation|GetActorLocation TargetActor) (Transformation|GetActorLocation SourceActor)) 0.0001)))

(fn 设置角色朝向
  (params (设置旋转的目标 :type Actor%20Object%20Reference) (Orientation :type Vector))
  (Transformation|SetActorRotation 设置旋转的目标 (Math|Conversions|RotationFromXVector Orientation)))

(fn 概率产生器与随机数产生器
  (params (所需概率 :type Float%20%28double-precision%29))
  (bind _returnvalue (Math|Random|RandomFloatinRange 0.0 1e+02))
  (bind _returnvalue_2 (> 所需概率 _returnvalue))
  (if _returnvalue_2
    (return _returnvalue_2 _returnvalue)
    (else
      (return _returnvalue_2 _returnvalue))))

(fn 获取Actor周围一个随机点2D
  (params (Actor :type Actor%20Object%20Reference) (半径 :type Integer))
  (bind _returnvalue (Transformation|GetActorLocation Actor))
  (bind _returnvalue_2 (Math|Random|RandomUnitVector))
  (bind _returnvalue_3 (Math|Random|RandomInteger 半径))
  (bind _returnvalue_4 (* _returnvalue_2 _returnvalue_3))
  (bind _returnvalue_5 (+ _returnvalue _returnvalue_4))
  (return (Math|Vector|MakeVector (.x _returnvalue_5) (.y _returnvalue_5) 0.0)))