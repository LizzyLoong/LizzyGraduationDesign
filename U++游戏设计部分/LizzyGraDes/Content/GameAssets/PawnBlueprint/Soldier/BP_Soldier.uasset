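; Soldier pawn Blueprint that keeps its HP bar current and plays a hit reaction when it takes heavy damage.
; On BeginPlay it binds to HP and max HP change events; both handlers send the new value divided by an attribute value to the HP bar widget.
; HP changes also feed 小兵受击动画, which plays the hit montage when the drop exceeds a fixed threshold.
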(event Custom|HPChangeEvent_事件_0
  (params (OldValue :type Float%20%28single-precision%29) (NewValue :type Float%20%28single-precision%29))
  (Class|BPIWBPStateBar|BPIUpdateHP(Message) (UserInterface|GetUserWidgetObject (Variables|Default|GetHPBar)) (/ NewValue (CallFunction|GetAttributeValue "(AttributeName=\"MaxHP\",Attribute=/Script/LizzyGraDes.CPP_BaseAttributeSet:MaxHP,AttributeOwner=\"/Script/CoreUObject.Class'/Script/LizzyGraDes.CPP_BaseAttributeSet'\")")))
  (|小兵受击动画 OldValue NewValue))

(event Custom|MaxHPChangeEvent_事件_0
  (params (OldValue :type Float%20%28single-precision%29) (NewValue :type Float%20%28single-precision%29))
  (Class|BPIWBPStateBar|BPIUpdateHP(Message) (UserInterface|GetUserWidgetObject (Variables|Default|GetHPBar)) (/ NewValue (CallFunction|GetAttributeValue "(AttributeName=\"MaxHP\",Attribute=/Script/LizzyGraDes.CPP_BaseAttributeSet:MaxHP,AttributeOwner=\"/Script/CoreUObject.Class'/Script/LizzyGraDes.CPP_BaseAttributeSet'\")"))))

(event EventBeginPlay
  (|CallParentFunction)
  (EventDispatchers|AssignHPChangeEvent (delegate Custom|HPChangeEvent_事件_0))
  (EventDispatchers|AssignMaxHPChangeEvent (delegate Custom|MaxHPChangeEvent_事件_0)))

(event Collision|EventActorBeginOverlap
  (params (OtherActor :type Actor%20Object%20Reference))
  (|CallParentFunction OtherActor) ; 此节点被禁用，将不会被调用。\n从引脚连出引线来编译功能。
)

(fn ConstructionScript
  (|CallParentFunction))