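; BP_BaseGem is a gem Blueprint that picks a random gem variant when constructed.
; Its Construction Script runs a chain of threshold checks on 概率产生器与随机数产生器's random number within 100, evaluated again at each check.
; The passing branch sets the static mesh, ore type (矿石种类) and quality tier (矿石品质), from black through colorful.
; The event graph holds only disabled stub events.
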(event EventBeginPlay)

(event Collision|EventActorBeginOverlap
  (params (OtherActor :type Actor%20Object%20Reference)))

(event EventTick
  (params (DeltaSeconds :type Float%20%28single-precision%29)))

(fn ConstructionScript
  (bind _100以内的随机数 (CallFunction|概率产生器与随机数产生器 0.0))
  (bind _returnvalue (Math|Float|Truncate _100以内的随机数))
  (if (<= _returnvalue 1)
    (Components|StaticMesh|SetStaticMesh (Variables|Default|GetStaticMesh) "/Game/GameAssets/PawnBlueprint/Gem/Assets/GemBlack.GemBlack")
    (Variables|Default|Set矿石种类 "NewEnumerator0")
    (Variables|Default|Set矿石品质 "NewEnumerator0")
    (elif (<= _returnvalue 2)
      (Components|StaticMesh|SetStaticMesh (Variables|Default|GetStaticMesh) "/Game/GameAssets/PawnBlueprint/Gem/Assets/GemWhite.GemWhite")
      (Variables|Default|Set矿石种类 "NewEnumerator1")
      (Variables|Default|Set矿石品质 "NewEnumerator0")
      (elif (<= _returnvalue 4)
        (Components|StaticMesh|SetStaticMesh (Variables|Default|GetStaticMesh) "/Game/GameAssets/PawnBlueprint/Gem/Assets/GemFloating.GemFloating")
        (Variables|Default|Set矿石种类 "NewEnumerator8")
        (Variables|Default|Set矿石品质 "NewEnumerator0")
        (elif (<= _returnvalue 6)
          (Components|StaticMesh|SetStaticMesh (Variables|Default|GetStaticMesh) "/Game/GameAssets/PawnBlueprint/Gem/Assets/GemParcel.GemParcel")
          (Variables|Default|Set矿石种类 "NewEnumerator9")
          (Variables|Default|Set矿石品质 "NewEnumerator0")
          (elif (<= _returnvalue 11)
            (Components|StaticMesh|SetStaticMesh (Variables|Default|GetStaticMesh) "/Game/GameAssets/PawnBlueprint/Gem/Assets/GemRed.GemRed")
            (Variables|Default|Set矿石种类 "NewEnumerator2")
            (Variables|Default|Set矿石品质 "NewEnumerator1")
            (elif (<= _returnvalue 16)
              (Components|StaticMesh|SetStaticMesh (Variables|Default|GetStaticMesh) "/Game/GameAssets/PawnBlueprint/Gem/Assets/GemGreen.GemGreen")
              (Variables|Default|Set矿石种类 "NewEnumerator3")
              (Variables|Default|Set矿石品质 "NewEnumerator1")
              (elif (<= _returnvalue 21)
                (Components|StaticMesh|SetStaticMesh (Variables|Default|GetStaticMesh) "/Game/GameAssets/PawnBlueprint/Gem/Assets/GemBlue.GemBlue")
                (Variables|Default|Set矿石种类 "NewEnumerator4")
                (Variables|Default|Set矿石品质 "NewEnumerator1")
                (elif (<= _returnvalue 31)
                  (Components|StaticMesh|SetStaticMesh (Variables|Default|GetStaticMesh) "/Game/GameAssets/PawnBlueprint/Gem/Assets/GemPurple.GemPurple")
                  (Variables|Default|Set矿石种类 "NewEnumerator5")
                  (Variables|Default|Set矿石品质 "NewEnumerator2")
                  (elif (<= _returnvalue 41)
                    (Components|StaticMesh|SetStaticMesh (Variables|Default|GetStaticMesh) "/Game/GameAssets/PawnBlueprint/Gem/Assets/GemGolden.GemGolden")
                    (Variables|Default|Set矿石种类 "NewEnumerator6")
                    (Variables|Default|Set矿石品质 "NewEnumerator2")
                    (elif (<= _returnvalue 100)
                      (Components|StaticMesh|SetStaticMesh (Variables|Default|GetStaticMesh) "/Game/GameAssets/PawnBlueprint/Gem/Assets/GemColorful.GemColorful")
                      (Variables|Default|Set矿石种类 "NewEnumerator10")
                      (Variables|Default|Set矿石品质 "NewEnumerator3"))))))))))))