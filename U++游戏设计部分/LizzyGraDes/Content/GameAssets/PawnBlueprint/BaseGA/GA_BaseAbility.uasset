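; GA_BaseAbility is a base Gameplay Ability offering shared movement helpers, with empty activate and end events.
; Flash offsets an actor along its forward vector without sweep.
; Dash (marked deprecated), Air and AirDash apply scaled CharacterMovement impulses to the owner, along its movement direction or up vector.
; 是否穿透Pawn toggles player 0's capsule between overlapping and blocking Pawns; a cooldown debug print is left unconnected.
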(event Custom|Dash%28逐渐废弃%29
  (params (距离 :type Integer))
  (bind _asbp_base_character (Utilities|Casting|CastToBP_BaseCharacter (.OwnerActor (Utilities|Struct|BreakGameplayAbilityActorInfo (Ability|GetActorInfo)))))
  (Physics|AddImpulse (Variables|/Script/Engine.Character|GetCharacterMovement _asbp_base_character) (* (Default|获取运动方向 _asbp_base_character) (* 距离 200000)) false))

(event Custom|AirDash
  (params (距离 :type Integer))
  (bind _asbp_base_character (Utilities|Casting|CastToBP_BaseCharacter (.OwnerActor (Utilities|Struct|BreakGameplayAbilityActorInfo (Ability|GetActorInfo)))))
  (Physics|AddImpulse (Variables|/Script/Engine.Character|GetCharacterMovement _asbp_base_character) (* (Default|获取运动方向 _asbp_base_character) (* 距离 16667)) false))

(event Custom|Flash
  (params (Actor :type Actor%20Object%20Reference) (Length :type Integer))
  (Transformation|SetActorLocation Actor (+ (* (Transformation|GetActorForwardVector Actor) Length) (Transformation|GetActorLocation Actor)) false false))

(event Custom|Air
  (params (高度 :type Integer))
  (bind _basecharacter (Class|BPIBaseGameplayMessage|TrytoGetBaseCharacter(Message) (.OwnerActor (Utilities|Struct|BreakGameplayAbilityActorInfo (Ability|GetActorInfo)))))
  (Physics|AddImpulse (Variables|/Script/Engine.Character|GetCharacterMovement _basecharacter) (* (Transformation|GetActorUpVector _basecharacter) (* 高度 30000)) false))

(event Ability|EventActivateAbility)

(event Ability|EventOnEndAbility
  (params (bWasCancelled :type Boolean)))

(fn 是否穿透Pawn
  (params (是 :type Boolean))
  (bind _returnvalue (Game|GetPlayerCharacter 0))
  (bind _capsulecomponent (Variables|/Script/Engine.Character|GetCapsuleComponent _returnvalue))
  (if 是
    (Collision|SetCollisionResponsetoChannel _capsulecomponent "ECC_Pawn" "ECR_Overlap")
    (else
      (Collision|SetCollisionResponsetoChannel _capsulecomponent "ECC_Pawn" "ECR_Block"))))