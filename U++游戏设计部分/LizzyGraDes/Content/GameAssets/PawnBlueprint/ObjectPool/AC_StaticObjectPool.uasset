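; AC_StaticObjectPool is an object pool component that pre-spawns actors for reuse instead of spawning them on demand.
; At BeginPlay it spawns PooledActorClass instances at the owner's transform based on PooledSize, marks them not in use, and stores them in PooledActors.
; SpawnFromPool linearly searches for an idle actor, moves it to the requested transform and marks it in use.
; The pool never grows, and an invalid search result only prints a failure message.
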(event EventBeginPlay
  (bind _returnvalue (Components|GetOwner))
  (for _index (range 0 (Variables|ObjectPool配置|GetPooledSize))
    (bind _returnvalue_2 (Game|SpawnActorfromClass (Variables|ObjectPool配置|GetPooledActorClass) (Transformation|GetActorTransform _returnvalue) "Undefined" "MultiplyWithRoot" _returnvalue 0))
    (Default|SetinUse _returnvalue_2 false)
    (Utilities|Array|AddUnique (Variables|ObjectPool配置|GetPooledActors) _returnvalue_2)))

(event EventTick
  (params (DeltaSeconds :type Float%20%28single-precision%29)))

(fn FindFirstAvaliableActor
  (bind _array_element (Utilities|Array|ForEachLoopwithBreak (Variables|ObjectPool配置|GetPooledActors) :!label _label)
    (:LoopBody
      (if (not (Variables|/Game/GameAssets/PawnBlueprint/ObjectPool/BP_PooledActor.BP_PooledActor_C|GetInUse _array_element))
        (goto _label Break)))
    (:Completed
      (return _array_element))))

(fn SpawnfromPool
  (params (SpawnTransform :type Transform))
  (bind _array_element (CallFunction|FindFirstAvaliableActor))
  (Utilities|IsValid _array_element
    (:Is%20Valid
      (Transformation|SetActorTransform _array_element SpawnTransform)
      (Default|SetinUse _array_element true)
      (return _array_element))
    (:Is%20Not%20Valid
      (Development|PrintText "从池中生成失败"))))