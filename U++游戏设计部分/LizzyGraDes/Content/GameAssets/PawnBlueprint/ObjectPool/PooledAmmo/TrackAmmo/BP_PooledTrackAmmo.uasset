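; BP_PooledTrackAmmo is a pooled homing projectile, judging by its name and folder.
; Its SetHoming event enables homing on AmmoMovement, targets the given actor's Mesh component and sets a fixed homing acceleration.
; Both sides of the validity check do the same thing, so an invalid target's Mesh is still read.
; BeginPlay, overlap and Tick are disabled stubs, and the construction script only calls its parent.
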(event Custom|SetHoming
  (params (TargetActor :type BP%20Base%20Character%20Object%20Reference))
  (Utilities|IsValid TargetActor
    (:Is%20Valid
      (Variables|/Script/Engine.ProjectileMovementComponent|SetbIsHomingProjectile (Variables|Default|GetAmmoMovement) true)
      (Variables|/Script/Engine.ProjectileMovementComponent|SetHomingTargetComponent (Variables|Default|GetAmmoMovement) (Variables|/Script/Engine.Character|GetMesh TargetActor))
      (Variables|/Script/Engine.ProjectileMovementComponent|SetHomingAccelerationMagnitude (Variables|Default|GetAmmoMovement) 1e+04))
    (:Is%20Not%20Valid
      (Variables|/Script/Engine.ProjectileMovementComponent|SetbIsHomingProjectile (Variables|Default|GetAmmoMovement) true)
      (Variables|/Script/Engine.ProjectileMovementComponent|SetHomingTargetComponent (Variables|Default|GetAmmoMovement) (Variables|/Script/Engine.Character|GetMesh (Variables|Default|GetTargetActor)))
      (Variables|/Script/Engine.ProjectileMovementComponent|SetHomingAccelerationMagnitude (Variables|Default|GetAmmoMovement) 1e+04))))

(event EventBeginPlay
  (|CallParentFunction) ; 此节点被禁用，将不会被调用。\n从引脚连出引线来编译功能。
)

(event Collision|EventActorBeginOverlap
  (params (OtherActor :type Actor%20Object%20Reference))
  (|CallParentFunction OtherActor) ; 此节点被禁用，将不会被调用。\n从引脚连出引线来编译功能。
)

(event EventTick
  (params (DeltaSeconds :type Float%20%28single-precision%29))
  (|CallParentFunction DeltaSeconds) ; 此节点被禁用，将不会被调用。\n从引脚连出引线来编译功能。
)

(fn ConstructionScript
  (|CallParentFunction))