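; BP_BaseGameInstance is a base Game Instance that caches the Player 0 pawn and exposes shared lookup functions.
; TryToSetPlayer0Pawn stores the given pawn and returns it, while TryToGetPlayer0Pawn reads the cached reference.
; The BPI functions for game mode, can-buy and purchase condition, along with TryToGetBaseCharacter, are stubs that return empty or false values.
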(fn BPIGetBaseGameMode
  (return 0))

(fn BPIGetCanBuy
  (return false))

(fn BPIGetPurchaseCondition
  (return false))

(fn TrytoGetBaseCharacter
  (return 0))

(fn TrytoGetPlayer0Pawn
  (return (Variables|Default|GetPlayer0Pawn)))

(fn TrytoSetPlayer0Pawn
  (params (ControlledPawn :type BP%20Base%20Character%20Class%20Reference))
  (bind _output_get (Variables|Default|SetPlayer0Pawn ControlledPawn))
  (return _output_get))