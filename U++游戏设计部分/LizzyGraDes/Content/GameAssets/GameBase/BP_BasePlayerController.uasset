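; Base player controller that sets up input and UI and tracks whether the player can buy.
; A short timer after BeginPlay adds mapping contexts, caches the controlled character, and creates main, shop and bag widgets.
; CanBuy is read from the game mode through interface calls and refreshed by its purchase-condition dispatcher.
; Input toggles bag and shop together and switches to a grab-hand cursor during select; several getter/setter functions are empty stubs.
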(event Custom|自定义事件
  (Utilities|FlowControl|Sequence
    (:then_0
      (|增强输入))
    (:then_1
      (|锁定初始角色并创建其UI))
    (:then_2
      (|ShopUI和BagUI))
    (:then_3
      (bind _是否可以购买 (Class|BPIBaseGameplayMessage|BPIGetPurchaseCondition(Message) (Game|GetGameMode)))
      (Variables|Default|SetCanBuy _是否可以购买)
      (bind _basegamemode (Class|BPIBaseGameplayMessage|BPIGetBaseGameMode(Message) (Game|GetGameMode)))
      (EventDispatchers|AssignOnPurchaseConditionChange _basegamemode (delegate Custom|OnPurchaseConditionChange_事件)))))

(event Custom|OnPurchaseConditionChange_事件
  (bind _是否可以购买 (Class|BPIBaseGameplayMessage|BPIGetPurchaseCondition(Message) (Game|GetGameMode)))
  (Variables|Default|SetCanBuy _是否可以购买))

(event Input|EnhancedActionEvents|EnhancedInputActionInteract_SelectAndVerify
  (params (ActionValue :type Boolean) (ElapsedSeconds :type Float%20%28double-precision%29) (TriggeredSeconds :type Float%20%28double-precision%29) (InputAction :type Input%20Action%20Object%20Reference :default "/Game/GameAssets/Input/Interact/Interact_SelectAndVerify.Interact_SelectAndVerify"))
  (:Triggered
    (Variables|Default|SetCurrentMouseCursor "GrabHand" :!label _label))
  (:Started
    (goto _label))
  (:Ongoing
    (Variables|Default|SetCurrentMouseCursor "Default" :!label _label_2))
  (:Canceled
    (goto _label_2))
  (:Completed
    (goto _label_2)))

(event Input|EnhancedActionEvents|EnhancedInputActionInteract_OpenBag
  (params (ActionValue :type Boolean) (ElapsedSeconds :type Float%20%28double-precision%29) (TriggeredSeconds :type Float%20%28double-precision%29) (InputAction :type Input%20Action%20Object%20Reference :default "/Game/GameAssets/Input/Interact/Interact_OpenBag.Interact_OpenBag"))
  (:Started
    (Default|HandleWidgetSwitch (Variables|Default|GetBagUI))
    (Default|HandleWidgetSwitch (Variables|Default|GetShopUI))))

(event EventBeginPlay
  (Utilities|Time|SetTimerbyEvent (delegate Custom|自定义事件) 0.5))

(fn ConstructionScript)

(fn BPIGetBaseGameMode
  (return 0))

(fn BPIGetCanBuy
  (return (Variables|Default|GetCanBuy)))

(fn BPIGetPurchaseCondition
  (return false))

(fn TrytoGetBaseCharacter
  (return (Variables|Default|GetDefaultCharacter)))

(fn TrytoGetPlayer0Pawn
  (return 0))

(fn TrytoSetPlayer0Pawn
  (params (ControlledPawn :type BP%20Base%20Character%20Class%20Reference))
  (return 0))