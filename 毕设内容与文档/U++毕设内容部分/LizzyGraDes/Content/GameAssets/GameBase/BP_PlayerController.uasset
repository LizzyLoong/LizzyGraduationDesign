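; Player controller that sets up Enhanced Input, creates the main, bag and shop UI, and handles interaction input.
; A delayed timer after BeginPlay adds the character and interact mapping contexts, shows the main UI, and passes the controlled BP_BaseCharacter to it and the bag.
; The select input toggles the cursor between grab hand and default, while the open-bag input switches both bag and shop widgets together.
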(event Custom|自定义事件
  (bind _self self)
  (bind _returnvalue (PlayerController|LocalPlayerSubsystems|GetEnhancedInputLocalPlayerSubsystem _self))
  (Utilities|FlowControl|Sequence
    (:then_0
      (Utilities|IsValid _returnvalue
        (:Is%20Valid
          (Input|AddMappingContext _returnvalue "/Game/GameAssets/Input/IMC_CharacterControl_IsShortForCC.IMC_CharacterControl_IsShortForCC" 0 "(bIgnoreAllPressedKeysUntilRelease=True,bForceImmediately=False,bNotifyUserSettings=False)")
          (Input|AddMappingContext _returnvalue "/Game/GameAssets/Input/IMC_Interact.IMC_Interact" 1 "(bIgnoreAllPressedKeysUntilRelease=True,bForceImmediately=False,bNotifyUserSettings=False)")
          (bind _returnvalue_2 (UserInterface|CreateWidget "/Game/GameAssets/PawnBlueprint/UI/WBP_MainUI.WBP_MainUI_C"))
          (bind _output_get (Variables|Default|SetWidgetMainUI _returnvalue_2))
          (UserInterface|Viewport|AddtoViewport _output_get 0))))
    (:then_1
      (bind _asbp_base_character (Utilities|Casting|CastToBP_BaseCharacter (Pawn|GetControlledPawn)))
      (bind _output_get_2 (Variables|Default|SetAs%20BP%20Base%20Character _asbp_base_character))
      (Default|InitUI (Variables|Default|GetWidgetMainUI) _output_get_2)
      (bind _returnvalue_3 (UserInterface|CreateWidget "/Game/GameAssets/PawnBlueprint/EquipmentSystem/BagItem/WBP_Bag.WBP_Bag_C" self _output_get_2))
      (Variables|Default|SetBagUI _returnvalue_3))
    (:then_2
      (bind _returnvalue_4 (UserInterface|CreateWidget "/Game/GameAssets/PawnBlueprint/EquipmentSystem/Shop/WBP_Shop.WBP_Shop_C" self))
      (Variables|Default|SetShopUI _returnvalue_4))))

(event Input|EnhancedActionEvents|EnhancedInputActionInteract_SelectAndVerify
  (params (ActionValue :type Boolean) (ElapsedSeconds :type Float%20%28double-precision%29) (TriggeredSeconds :type Float%20%28double-precision%29) (InputAction :type Input%20Action%20Object%20Reference :default "/Game/GameAssets/Input/Interact/Interact_SelectAndVerify.Interact_SelectAndVerify"))
  (:Triggered
    (Variables|Default|SetCurrentMouseCursor "GrabHand" :!label _label))
  (:Started
    (goto _label))
  (:Ongoing
    (Variables|Default|SetCurrentMouseCursor "Default" :!label _label_2))
  (:Canceled
    (goto _label_2))
  (:Completed
    (goto _label_2)))

(event Input|EnhancedActionEvents|EnhancedInputActionInteract_OpenBag
  (params (ActionValue :type Boolean) (ElapsedSeconds :type Float%20%28double-precision%29) (TriggeredSeconds :type Float%20%28double-precision%29) (InputAction :type Input%20Action%20Object%20Reference :default "/Game/GameAssets/Input/Interact/Interact_OpenBag.Interact_OpenBag"))
  (:Started
    (Default|HandleBagSwitch (Variables|Default|GetBagUI))
    (Default|HandleShopSwitch (Variables|Default|GetShopUI))))

(event EventBeginPlay
  (Utilities|Time|SetTimerbyEvent (delegate Custom|自定义事件) 0.5))

(fn ConstructionScript)