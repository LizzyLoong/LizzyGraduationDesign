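; Legends pawn Blueprint that keeps its StateBar widget in sync with the pawn's HP, MP and SP attributes.
; On BeginPlay, separate HP, MP and SP graphs bind handlers to each attribute's current and max change events.
; Each handler divides the new value by a queried attribute value and sends the ratio to the widget through an interface message, avoiding per-tick polling.
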(event EventBeginPlay
  (|CallParentFunction)
  (|HP)
  (|MP)
  (|SP))

(event Collision|EventActorBeginOverlap
  (params (OtherActor :type Actor%20Object%20Reference))
  (|CallParentFunction OtherActor) ; 此节点被禁用，将不会被调用。\n从引脚连出引线来编译功能。
)

(event EventTick
  (params (DeltaSeconds :type Float%20%28single-precision%29))
  (|CallParentFunction DeltaSeconds))

(fn ConstructionScript
  (|CallParentFunction))

(event Custom|MPChangeEvent_事件_0
  (params (OldValue :type Float%20%28single-precision%29) (NewValue :type Float%20%28single-precision%29))
  (Class|BPIWBPStateBar|BPIUpdateMP(Message) (UserInterface|GetUserWidgetObject (Variables|Default|GetStateBar)) (/ NewValue (CallFunction|GetAttributeValue "(AttributeName=\"MaxMP\",Attribute=/Script/LizzyGraDes.CPP_BaseAttributeSet:MaxMP,AttributeOwner=\"/Script/CoreUObject.Class'/Script/LizzyGraDes.CPP_BaseAttributeSet'\")"))))

(event Custom|MaxMPChangeEvent_事件_0
  (params (OldValue :type Float%20%28single-precision%29) (NewValue :type Float%20%28single-precision%29))
  (Class|BPIWBPStateBar|BPIUpdateMP(Message) (UserInterface|GetUserWidgetObject (Variables|Default|GetStateBar)) (/ NewValue (CallFunction|GetAttributeValue "(AttributeName=\"MaxMP\",Attribute=/Script/LizzyGraDes.CPP_BaseAttributeSet:MaxMP,AttributeOwner=\"/Script/CoreUObject.Class'/Script/LizzyGraDes.CPP_BaseAttributeSet'\")"))))

(event Custom|SPChangeEvent_事件_0
  (params (OldValue :type Float%20%28single-precision%29) (NewValue :type Float%20%28single-precision%29))
  (Class|BPIWBPStateBar|BPIUpdateSP(Message) (UserInterface|GetUserWidgetObject (Variables|Default|GetStateBar)) (/ NewValue (CallFunction|GetAttributeValue "(AttributeName=\"MaxSP\",Attribute=/Script/LizzyGraDes.CPP_BaseAttributeSet:MaxSP,AttributeOwner=\"/Script/CoreUObject.Class'/Script/LizzyGraDes.CPP_BaseAttributeSet'\")"))))

(event Custom|MaxSPChangeEvent_事件_0
  (params (OldValue :type Float%20%28single-precision%29) (NewValue :type Float%20%28single-precision%29))
  (Class|BPIWBPStateBar|BPIUpdateSP(Message) (UserInterface|GetUserWidgetObject (Variables|Default|GetStateBar)) (/ NewValue (CallFunction|GetAttributeValue "(AttributeName=\"MaxSP\",Attribute=/Script/LizzyGraDes.CPP_BaseAttributeSet:MaxSP,AttributeOwner=\"/Script/CoreUObject.Class'/Script/LizzyGraDes.CPP_BaseAttributeSet'\")"))))

(event Custom|HPChangeEvent_事件_0
  (params (OldValue :type Float%20%28single-precision%29) (NewValue :type Float%20%28single-precision%29))
  (Class|BPIWBPStateBar|BPIUpdateHP(Message) (UserInterface|GetUserWidgetObject (Variables|Default|GetStateBar)) (/ NewValue (CallFunction|GetAttributeValue "(AttributeName=\"MaxHP\",Attribute=/Script/LizzyGraDes.CPP_BaseAttributeSet:MaxHP,AttributeOwner=\"/Script/CoreUObject.Class'/Script/LizzyGraDes.CPP_BaseAttributeSet'\")"))))

(event Custom|MaxHPChangeEvent_事件_0
  (params (OldValue :type Float%20%28single-precision%29) (NewValue :type Float%20%28single-precision%29))
  (Class|BPIWBPStateBar|BPIUpdateHP(Message) (UserInterface|GetUserWidgetObject (Variables|Default|GetStateBar)) (/ NewValue (CallFunction|GetAttributeValue "(AttributeName=\"MaxHP\",Attribute=/Script/LizzyGraDes.CPP_BaseAttributeSet:MaxHP,AttributeOwner=\"/Script/CoreUObject.Class'/Script/LizzyGraDes.CPP_BaseAttributeSet'\")"))))