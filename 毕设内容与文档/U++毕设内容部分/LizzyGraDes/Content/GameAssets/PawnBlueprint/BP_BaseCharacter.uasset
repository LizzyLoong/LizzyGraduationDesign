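; Base character Blueprint built on the Gameplay Ability System, with input-driven movement and facing.
; BeginPlay activates a recovery ability and binds equipment and attribute events: Run sets walk speed, Tough scales the capsule, HP drops spawn damage widgets.
; Cursor hover applies an overlay highlight, and interact input picks a BP_Legends under the cursor as attack target.
; Helpers provide launch and dash impulses and ground traces; debug keys toggle a prediction/advice widget.
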(event OnBeginCursorOver(Mesh)
  (params (TouchedComponent :type Primitive%20Component%20Object%20Reference))
  (Rendering|Material|SetOverlayMaterial (Variables|Character|GetMesh) "/Game/GameAssets/PawnBlueprint/UI/Cursor/Highlight/MI_EnemyHighlight.MI_EnemyHighlight" :!class /Script/Engine.MeshComponent))

(event OnEndCursorOver(Mesh)
  (params (TouchedComponent :type Primitive%20Component%20Object%20Reference))
  (Rendering|Material|SetOverlayMaterial (Variables|Character|GetMesh) 0 :!class /Script/Engine.MeshComponent))

(event Custom|HPChangeEvent_事件
  (params (OldValue :type Float%20%28single-precision%29) (NewValue :type Float%20%28single-precision%29))
  (bind _returnvalue (- OldValue NewValue))
  (if (and (<= OldValue (CallFunction|GetAttributeValue "(AttributeName=\"MaxHP\",Attribute=/Script/LizzyGraDes.CPP_BaseAttributeSet:MaxHP,AttributeOwner=\"/Script/CoreUObject.Class'/Script/LizzyGraDes.CPP_BaseAttributeSet'\")")) (> _returnvalue 1.0))
    (bind _returnvalue_2 (UserInterface|CreateWidget "/Game/GameAssets/PawnBlueprint/UI/WBP_DamageShow.WBP_DamageShow_C" 0 _returnvalue))
    (Class|UserWidget|SetPositioninViewport _returnvalue_2 (.ScreenPosition (Class|GameplayStatics|ProjectWorldtoScreen (Game|GetPlayerController 0) (Transformation|GetActorLocation self) false)) true)
    (UserInterface|Viewport|AddtoViewport _returnvalue_2 0)))

(event Custom|OnEquipmentUpdate_事件
  (Class|CPPBaseCharacter|SetCharacterAttributeComment))

(event Input|EnhancedActionEvents|EnhancedInputActionInteract_SelectAndVerify
  (params (ActionValue :type Boolean) (ElapsedSeconds :type Float%20%28double-precision%29) (TriggeredSeconds :type Float%20%28double-precision%29) (InputAction :type Input%20Action%20Object%20Reference :default "/Game/GameAssets/Input/Interact/Interact_SelectAndVerify.Interact_SelectAndVerify"))
  (:Started
    (bind _asbp_legends (Utilities|Casting|CastToBP_Legends (.HitActor (Collision|BreakHitResult (.HitResult (Game|Player|GetHitResultUnderCursorbyChannel (Game|GetPlayerController 0) "TraceTypeQuery1" true))))))
    (Variables|Default|SetAttackTargetActor _asbp_legends)
    (Default|CallOnTargetActorChange)
    (Development|PrintText (Utilities|Text|ToText(Object) (Variables|Default|GetAttackTargetActor)))))

(event EventBeginPlay
  (|CallParentFunction)
  (Utilities|FlowControl|Sequence
    (:then_0
      (bind _asbp_player_controller (Utilities|Casting|CastToBP_PlayerController (Game|GetPlayerController 0)))
      (Variables|Default|SetAs%20BP%20Player%20Controller _asbp_player_controller)
      (Variables|Default|SetActor半高 (.z (Transformation|GetWorldLocation (Variables|Default|GetFootTransform)))))
    (:then_1
      (|WalkSpeedUpdate)
      (|ScaleUpdate))
    (:then_2
      (Class|AbilitySystemComponent|GiveAbilityandActivateOnce (Variables|Default|GetAbilitySystem) "/Game/GameAssets/PawnBlueprint/GA_BaseRecover.GA_BaseRecover_C" 0 -1)
      (EventDispatchers|AssignOnEquipmentUpdate (Variables|Default|GetEquipmentSystem) (delegate Custom|OnEquipmentUpdate_事件)))
    (:then_3
      (EventDispatchers|AssignHPChangeEvent (delegate Custom|HPChangeEvent_事件)))))

(event Collision|EventActorBeginOverlap
  (params (OtherActor :type Actor%20Object%20Reference)))

(event Input|KeyboardEvents|DebugKeyB
  (params (Key :type Key%20Structure :default "None") (ActionValue :type Input%20Action%20Value%20Structure)))

(event Input|KeyboardEvents|DebugKeyB
  (params (Key :type Key%20Structure :default "None") (ActionValue :type Input%20Action%20Value%20Structure))
  (:Pressed
    (bind _returnvalue (UserInterface|CreateWidget "/Game/GameAssets/PawnBlueprint/UI/WBP_CallPredictAndGetAdvice.WBP_CallPredictAndGetAdvice_C" 0 self))
    (UserInterface|Viewport|AddtoViewport _returnvalue 0)))

(event Input|KeyboardEvents|DebugKeyV
  (params (Key :type Key%20Structure :default "None") (ActionValue :type Input%20Action%20Value%20Structure))
  (:Pressed
    (Widget|RemovefromParent (stale Input|KeyboardEvents|DebugKeyB _returnvalue))))

(event Input|EnhancedActionEvents|EnhancedInputActionCC_Move
  (params (ActionValue :type Vector%202D%20Structure) (ElapsedSeconds :type Float%20%28double-precision%29) (TriggeredSeconds :type Float%20%28double-precision%29) (InputAction :type Input%20Action%20Object%20Reference :default "/Game/GameAssets/Input/CC/CC_Move.CC_Move"))
  (Pawn|Input|AddMovementInput (Math|Vector|MakeVector (.x ActionValue) (.y ActionValue) 0.0) 1.0 false))

(event Input|EnhancedActionEvents|EnhancedInputActionCC_Rotate
  (params (ActionValue :type Vector%202D%20Structure) (ElapsedSeconds :type Float%20%28double-precision%29) (TriggeredSeconds :type Float%20%28double-precision%29) (InputAction :type Input%20Action%20Object%20Reference :default "/Game/GameAssets/Input/CC/CC_Rotate.CC_Rotate"))
  (CallFunction|设置角色朝向 self (Math|Vector|MakeVector (.x ActionValue) (.y ActionValue) 0.0)))

(fn ConstructionScript
  (Variables|/Script/Engine.CharacterMovementComponent|SetMaxWalkSpeed (Variables|Character|GetCharacterMovement) (CallFunction|GetAttributeValue "(AttributeName=\"Run\",Attribute=/Script/LizzyGraDes.CPP_BaseAttributeSet:Run,AttributeOwner=\"/Script/CoreUObject.Class'/Script/LizzyGraDes.CPP_BaseAttributeSet'\")"))
  (Variables|Default|SetActor半高 (.z (Transformation|GetWorldLocation (Variables|Default|GetFootTransform)))))

(fn 获取技能标签组中指定技能
  (params (组中Index :type Integer))
  (return (Utilities|Array|Get(acopy) (Variables|Default|Get技能标签组) 组中Index)))

(fn 获取运动方向
  (bind _returnvalue (Transformation|GetVelocity))
  (bind _returnvalue_2 (Class|KismetMathLibrary|VectorNormal2D _returnvalue 0.0001))
  (if (Utilities|Operators|EqualEqual :A _returnvalue_2)
    (return (Transformation|GetActorForwardVector))
    (else
      (return _returnvalue_2))))

(fn GetAttributeValue
  (params (Attribute :type Gameplay%20Attribute%20Structure))
  (return (.ReturnValue (Ability|Attribute|GetFloatAttributefromAbilitySystemComponent (Variables|Default|GetAbilitySystem) Attribute))))

(fn 起飞
  (params (击飞高度（给值建议1，2） :type Float%20%28double-precision%29))
  (Physics|AddImpulse (Variables|Character|GetCharacterMovement) (* (Transformation|GetActorUpVector) (* 击飞高度（给值建议1，2） 500)) true)
  (return))

(fn IsActoronGround
  (bind _foottransform (Variables|Default|GetFootTransform))
  (bind _returnvalue (Transformation|GetWorldLocation _foottransform))
  (bind (_outhit _returnvalue_2) (Collision|LineTraceByChannel _returnvalue (- _returnvalue (Math|Vector|MakeVector 0.0 0.0 (+ (Variables|Default|GetActor半高) 1e+01))) "TraceTypeQuery1" false 0 "Persistent"))
  (return _outhit _returnvalue_2))

(fn Dash
  (params (Direction（NeedToNormalize） :type Vector) (Dist :type Float%20%28double-precision%29))
  (Physics|AddImpulse (Variables|Character|GetCharacterMovement) (* Direction（NeedToNormalize） (* Dist 2e+05)) false))

(fn DashAir
  (params (Direction（NeedToNormalize） :type Vector) (Dist（以击飞高度1为单位） :type Float%20%28double-precision%29))
  (Physics|AddImpulse (Variables|Character|GetCharacterMovement) (* Direction（NeedToNormalize） (* Dist（以击飞高度1为单位） 1e+04)) false))

(event Custom|RunChangeEvent_事件
  (params (OldValue :type Float%20%28single-precision%29) (NewValue :type Float%20%28single-precision%29))
  (Variables|/Script/Engine.CharacterMovementComponent|SetMaxWalkSpeed (Variables|Character|GetCharacterMovement) NewValue))

(event Custom|ToughChangeEvent_事件
  (params (OldValue :type Float%20%28single-precision%29) (NewValue :type Float%20%28single-precision%29))
  (Transformation|SetWorldScale3D (Variables|Default|GetCapsuleComponent) (* "1.000000,1.000000,1.000000" (+ (/ NewValue 100) (.x (Transformation|GetActorScale3D)))))
  (Utilities|FlowControl|DelayUntilNextTick)
  (Variables|Default|SetActor半高 (.z (Transformation|GetWorldLocation (Variables|Default|GetFootTransform)))))