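; Actor component that keeps a fixed-size pool of pre-spawned actors for reuse in place of spawning on demand.
; On BeginPlay it spawns instances of the pooled class at the owner's transform and marks each as not in use.
; SpawnFromPool scans linearly for a free actor, moves it to the requested transform, marks it in use and returns it.
; The pool never grows after BeginPlay.
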(event EventBeginPlay
  (for _index (range 0 (Variables|Init配置|GetPooledSize))
    (bind _returnvalue (Game|SpawnActorfromClass (Variables|Init配置|GetPooledActorClass) (Transformation|GetActorTransform (Components|GetOwner)) "Undefined" "MultiplyWithRoot" 0 0))
    (Default|SetinUse _returnvalue false)
    (Utilities|Array|AddUnique (Variables|Init配置|GetPooledActors) _returnvalue)))

(event EventTick
  (params (DeltaSeconds :type Float%20%28single-precision%29)))

(fn FindFirstAvaliableActor
  (bind _array_element (Utilities|Array|ForEachLoopwithBreak (Variables|Init配置|GetPooledActors) :!label _label)
    (:LoopBody
      (if (not (Variables|/Game/GameAssets/PawnBlueprint/ObjectPool/BP_PooledActor.BP_PooledActor_C|GetInUse _array_element))
        (goto _label Break)))
    (:Completed
      (return _array_element))))

(fn SpawnfromPool
  (params (Transform :type Transform))
  (bind _array_element (CallFunction|FindFirstAvaliableActor))
  (Utilities|IsValid _array_element
    (:Is%20Valid
      (Transformation|SetActorTransform _array_element Transform)
      (Default|SetinUse _array_element true)
      (return _array_element))))