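; Equipment component managing a weapon slot and five elemental slots (metal, wood, water, fire, earth), a class-based bag and a carried resource for purchases.
; Equipping and unequipping move classes between slots and bag, then broadcast per-slot update dispatchers.
; Handlers, bound one second after BeginPlay, apply or remove each item's GameplayEffect and abilities on the owner's AbilitySystemComponent, activating abilities when granted.
; A half-second looping timer rebroadcasts the resource value.
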(event Custom|自定义事件
  (Default|CallOnResourceChange (Variables|Default|GetCarriedResource)))

(event Custom|将装备的属性、技能、变换绑定到角色上
  (|OnWeaponUpdate)
  (|OnJinUpdate)
  (|OnMuUpdate)
  (|OnShuiUpdate)
  (|OnHuoUpdate)
  (|OnTuUpdate))

(event EventBeginPlay
  (Utilities|Time|SetTimerbyEvent (delegate Custom|自定义事件) 0.5 true)
  (Utilities|Time|SetTimerbyEvent (delegate Custom|将装备的属性、技能、变换绑定到角色上) 1.0))

(event Custom|LoadUpEquipment
  (params (装备位置 :type E_EquipmentLocation%20Enum :default "NewEnumerator0") (Equipment :type BP%20Base%20Equipment%20Class%20Reference))
  (switch Utilities|FlowControl|Switch|SwitchonE_EquipmentLocation 装备位置
    (:NewEnumerator0
      (if (not (Utilities|IsValidClass (Variables|Equipment部分|Get武器位装备Class)))
        (BaseDeal|SettleEquipmentbyClass "NewEnumerator0" Equipment)
        (Utilities|Array|RemoveItem (Variables|Default|Get背包物品Class) Equipment)
        (Default|CallOnBagItemRefresh)))
    (:NewEnumerator1
      (if (not (Utilities|IsValidClass (Variables|Equipment部分|Get木位装备Class)))
        (BaseDeal|SettleEquipmentbyClass "NewEnumerator1" Equipment)
        (Utilities|Array|RemoveItem (Variables|Default|Get背包物品Class) Equipment)
        (Default|CallOnBagItemRefresh)))
    (:NewEnumerator2
      (if (not (Utilities|IsValidClass (Variables|Equipment部分|Get火位装备Class)))
        (BaseDeal|SettleEquipmentbyClass "NewEnumerator2" Equipment)
        (Utilities|Array|RemoveItem (Variables|Default|Get背包物品Class) Equipment)
        (Default|CallOnBagItemRefresh)))
    (:NewEnumerator3
      (if (not (Utilities|IsValidClass (Variables|Equipment部分|Get土位装备Class)))
        (BaseDeal|SettleEquipmentbyClass "NewEnumerator3" Equipment)
        (Utilities|Array|RemoveItem (Variables|Default|Get背包物品Class) Equipment)
        (Default|CallOnBagItemRefresh)))
    (:NewEnumerator4
      (if (not (Utilities|IsValidClass (Variables|Equipment部分|Get金位装备Class)))
        (BaseDeal|SettleEquipmentbyClass "NewEnumerator4" Equipment)
        (Utilities|Array|RemoveItem (Variables|Default|Get背包物品Class) Equipment)
        (Default|CallOnBagItemRefresh)))
    (:NewEnumerator5
      (if (not (Utilities|IsValidClass (Variables|Equipment部分|Get水位装备Class)))
        (BaseDeal|SettleEquipmentbyClass "NewEnumerator5" Equipment)
        (Utilities|Array|RemoveItem (Variables|Default|Get背包物品Class) Equipment)
        (Default|CallOnBagItemRefresh)))))

(event Custom|LoadDownEquipment
  (params (装备位置 :type E_EquipmentLocation%20Enum :default "NewEnumerator0"))
  (switch Utilities|FlowControl|Switch|SwitchonE_EquipmentLocation 装备位置
    (:NewEnumerator0
      (if (Utilities|IsValidClass (Variables|Equipment部分|Get武器位装备Class))
        (Utilities|Array|Add (Variables|Default|Get背包物品Class) (Variables|Equipment部分|Get武器位装备Class))
        (Default|CallOnBagItemRefresh)
        (Variables|Equipment部分|Set武器位装备Class 0)
        (Default|CallOnWeaponEquipmentUpdate)
        (Default|CallOnEquipmentUpdate)))
    (:NewEnumerator1
      (if (Utilities|IsValidClass (Variables|Equipment部分|Get木位装备Class))
        (Utilities|Array|Add (Variables|Default|Get背包物品Class) (Variables|Equipment部分|Get木位装备Class))
        (Default|CallOnBagItemRefresh)
        (Variables|Equipment部分|Set木位装备Class 0)
        (Default|CallOnMuEquipmentUpdate)
        (Default|CallOnEquipmentUpdate)))
    (:NewEnumerator2
      (if (Utilities|IsValidClass (Variables|Equipment部分|Get火位装备Class))
        (Utilities|Array|Add (Variables|Default|Get背包物品Class) (Variables|Equipment部分|Get火位装备Class))
        (Default|CallOnBagItemRefresh)
        (Variables|Equipment部分|Set火位装备Class 0)
        (Default|CallOnHuoEquipmentUpdate)
        (Default|CallOnEquipmentUpdate)))
    (:NewEnumerator3
      (if (Utilities|IsValidClass (Variables|Equipment部分|Get土位装备Class))
        (Utilities|Array|Add (Variables|Default|Get背包物品Class) (Variables|Equipment部分|Get土位装备Class))
        (Default|CallOnBagItemRefresh)
        (Variables|Equipment部分|Set土位装备Class 0)
        (Default|CallOnTuEquipmentUpdate)
        (Default|CallOnEquipmentUpdate)))
    (:NewEnumerator4
      (if (Utilities|IsValidClass (Variables|Equipment部分|Get金位装备Class))
        (Utilities|Array|Add (Variables|Default|Get背包物品Class) (Variables|Equipment部分|Get金位装备Class))
        (Default|CallOnBagItemRefresh)
        (Variables|Equipment部分|Set金位装备Class 0)
        (Default|CallOnJinEquipmentUpdate)
        (Default|CallOnEquipmentUpdate)))
    (:NewEnumerator5
      (if (Utilities|IsValidClass (Variables|Equipment部分|Get水位装备Class))
        (Utilities|Array|Add (Variables|Default|Get背包物品Class) (Variables|Equipment部分|Get水位装备Class))
        (Default|CallOnBagItemRefresh)
        (Variables|Equipment部分|Set水位装备Class 0)
        (Default|CallOnShuiEquipmentUpdate)
        (Default|CallOnEquipmentUpdate)))))

(fn SettleEquipmentbyClass
  (params (接入位置 :type E_EquipmentLocation%20Enum :default "NewEnumerator0") (装备 :type BP%20Base%20Equipment%20Class%20Reference))
  (switch Utilities|FlowControl|Switch|SwitchonE_EquipmentLocation 接入位置
    (:NewEnumerator0
      (if (Utilities|IsValidClass 装备)
        (Variables|Equipment部分|Set武器位装备Class 装备)
        (Default|CallOnWeaponEquipmentUpdate)
        (Default|CallOnEquipmentUpdate)))
    (:NewEnumerator1
      (if (Utilities|IsValidClass 装备)
        (Variables|Equipment部分|Set木位装备Class 装备)
        (Default|CallOnMuEquipmentUpdate)
        (Default|CallOnEquipmentUpdate)))
    (:NewEnumerator2
      (if (Utilities|IsValidClass 装备)
        (Variables|Equipment部分|Set火位装备Class 装备)
        (Default|CallOnHuoEquipmentUpdate)
        (Default|CallOnEquipmentUpdate)))
    (:NewEnumerator3
      (if (Utilities|IsValidClass 装备)
        (Variables|Equipment部分|Set土位装备Class 装备)
        (Default|CallOnTuEquipmentUpdate)
        (Default|CallOnEquipmentUpdate)))
    (:NewEnumerator4
      (if (Utilities|IsValidClass 装备)
        (Variables|Equipment部分|Set金位装备Class 装备)
        (Default|CallOnJinEquipmentUpdate)
        (Default|CallOnEquipmentUpdate)))
    (:NewEnumerator5
      (if (Utilities|IsValidClass 装备)
        (Variables|Equipment部分|Set水位装备Class 装备)
        (Default|CallOnShuiEquipmentUpdate)
        (Default|CallOnEquipmentUpdate)))))

(fn UnequipbyClass
  (params (装备位置 :type E_EquipmentLocation%20Enum :default "NewEnumerator0"))
  (switch Utilities|FlowControl|Switch|SwitchonE_EquipmentLocation 装备位置
    (:NewEnumerator0
      (if (Utilities|IsValidClass (Variables|Equipment部分|Get武器位装备Class))
        (Variables|Equipment部分|Set武器位装备Class 0)
        (Default|CallOnWeaponEquipmentUpdate)
        (Default|CallOnEquipmentUpdate)))
    (:NewEnumerator1
      (if (Utilities|IsValidClass (Variables|Equipment部分|Get木位装备Class))
        (Variables|Equipment部分|Set木位装备Class 0)
        (Default|CallOnMuEquipmentUpdate)
        (Default|CallOnEquipmentUpdate)))
    (:NewEnumerator2
      (if (Utilities|IsValidClass (Variables|Equipment部分|Get火位装备Class))
        (Variables|Equipment部分|Set火位装备Class 0)
        (Default|CallOnHuoEquipmentUpdate)
        (Default|CallOnEquipmentUpdate)))
    (:NewEnumerator3
      (if (Utilities|IsValidClass (Variables|Equipment部分|Get土位装备Class))
        (Variables|Equipment部分|Set土位装备Class 0)
        (Default|CallOnTuEquipmentUpdate)
        (Default|CallOnEquipmentUpdate)))
    (:NewEnumerator4
      (if (Utilities|IsValidClass (Variables|Equipment部分|Get金位装备Class))
        (Variables|Equipment部分|Set金位装备Class 0)
        (Default|CallOnJinEquipmentUpdate)
        (Default|CallOnEquipmentUpdate)))
    (:NewEnumerator5
      (if (Utilities|IsValidClass (Variables|Equipment部分|Get水位装备Class))
        (Variables|Equipment部分|Set水位装备Class 0)
        (Default|CallOnShuiEquipmentUpdate)
        (Default|CallOnEquipmentUpdate)))))

(fn BuyItembyClass
  (params (装备 :type BP%20Base%20Bag%20Item%20Class%20Reference))
  (bind _背包物品class (Variables|Default|Get背包物品Class))
  (bind _处理成功 (CallFunction|DealResource (* (Utilities|Struct|BreakS_BagItemAttribute (Utilities|GetClassDefaults 装备)) -1)))
  (if _处理成功
    (Default|CallOnBagItemRefresh)
    (bind _returnvalue (Utilities|Array|Add _背包物品class 装备))
    (for _array_element _背包物品class
      _)
    (return _returnvalue true)
    (else
      (return -1 false))))

(fn DealWeaponEquipmentAttributebyClass
  (bind _returnvalue (Components|GetOwner))
  (bind _武器位装备class (Variables|Equipment部分|Get武器位装备Class))
  (bind _returnvalue_2 (Ability|GetAbilitySystemComponent _returnvalue))
  (if (Utilities|IsValidClass _武器位装备class)
    (bind _returnvalue_3 (GameplayEffects|ApplyGameplayEffectToSelf :self _returnvalue_2 :GameplayEffectClass (.属性效果组 (Utilities|GetClassDefaults _武器位装备class))))
    (Variables|Equipment部分|Set武器位装备属性 _returnvalue_3)
    (else
      (GameplayEffects|RemoveActiveGameplayEffect _returnvalue_2 (Variables|Equipment部分|Get武器位装备属性) -1))))

(fn DealWeaponEquipmentAbilitybyClass
  (bind _武器位装备class (Variables|Equipment部分|Get武器位装备Class))
  (if (Utilities|IsValidClass _武器位装备class)
    (for _array_element (.技能能力组 (Utilities|GetClassDefaults _武器位装备class))
      (bind _returnvalue (GameplayAbilities|GiveAbility (Ability|GetAbilitySystemComponent (Components|GetOwner)) _array_element 0 -1))
      (Utilities|Array|Add (Variables|Equipment部分|Get武器位装备技能) _returnvalue)
      (Class|AbilitySystemComponent|TryActivateAbility (Ability|GetAbilitySystemComponent (Components|GetOwner)) _returnvalue true))
    (else
      (for _array_element_2 (Variables|Equipment部分|Get武器位装备技能)
        (GameplayAbilities|ClearAbility (Ability|GetAbilitySystemComponent (Components|GetOwner)) _array_element_2)
        (Utilities|Array|Clear (Variables|Equipment部分|Get武器位装备技能))))))

(fn DealJinEquipmentAbilitybyClass
  (bind _金位装备class (Variables|Equipment部分|Get金位装备Class))
  (if (Utilities|IsValidClass _金位装备class)
    (for _array_element (.技能能力组 (Utilities|GetClassDefaults _金位装备class))
      (bind _returnvalue (GameplayAbilities|GiveAbility (Ability|GetAbilitySystemComponent (Components|GetOwner)) _array_element 0 -1))
      (Utilities|Array|Add (Variables|Equipment部分|Get金位装备技能) _returnvalue)
      (Class|AbilitySystemComponent|TryActivateAbility (Ability|GetAbilitySystemComponent (Components|GetOwner)) _returnvalue true))
    (else
      (for _array_element_2 (Variables|Equipment部分|Get金位装备技能)
        (GameplayAbilities|ClearAbility (Ability|GetAbilitySystemComponent (Components|GetOwner)) _array_element_2)
        (Utilities|Array|Clear (Variables|Equipment部分|Get金位装备技能))))))

(fn DealResource
  (params (处理的Resource数量（花费请输入负数） :type Integer))
  (if (>= (+ 处理的Resource数量（花费请输入负数） (Variables|Default|GetCarriedResource)) 0)
    (bind _output_get (Variables|Default|SetCarriedResource (Math|Integer|Clamp(Integer) (+ 处理的Resource数量（花费请输入负数） (Variables|Default|GetCarriedResource)) 0 (Variables|Default|GetMaxCarriedResource))))
    (Default|CallOnResourceChange _output_get)
    (return true)
    (else
      (return false))))

(fn DealJinEquipmentAttributebyClass
  (bind _returnvalue (Components|GetOwner))
  (bind _金位装备class (Variables|Equipment部分|Get金位装备Class))
  (bind _returnvalue_2 (Ability|GetAbilitySystemComponent _returnvalue))
  (if (Utilities|IsValidClass _金位装备class)
    (bind _returnvalue_3 (GameplayEffects|ApplyGameplayEffectToSelf :self _returnvalue_2 :GameplayEffectClass (.属性效果组 (Utilities|GetClassDefaults _金位装备class))))
    (Variables|Equipment部分|Set金位装备属性 _returnvalue_3)
    (else
      (GameplayEffects|RemoveActiveGameplayEffect _returnvalue_2 (Variables|Equipment部分|Get金位装备属性) -1))))

(fn DealMuEquipmentAttributebyClass
  (bind _returnvalue (Components|GetOwner))
  (bind _木位装备class (Variables|Equipment部分|Get木位装备Class))
  (bind _returnvalue_2 (Ability|GetAbilitySystemComponent _returnvalue))
  (if (Utilities|IsValidClass _木位装备class)
    (bind _returnvalue_3 (GameplayEffects|ApplyGameplayEffectToSelf :self _returnvalue_2 :GameplayEffectClass (.属性效果组 (Utilities|GetClassDefaults _木位装备class))))
    (Variables|Equipment部分|Set木位装备属性 _returnvalue_3)
    (else
      (GameplayEffects|RemoveActiveGameplayEffect _returnvalue_2 (Variables|Equipment部分|Get木位装备属性) -1))))

(fn DealShuiEquipmentAttributebyClass
  (bind _returnvalue (Components|GetOwner))
  (bind _水位装备class (Variables|Equipment部分|Get水位装备Class))
  (bind _returnvalue_2 (Ability|GetAbilitySystemComponent _returnvalue))
  (if (Utilities|IsValidClass _水位装备class)
    (bind _returnvalue_3 (GameplayEffects|ApplyGameplayEffectToSelf :self _returnvalue_2 :GameplayEffectClass (.属性效果组 (Utilities|GetClassDefaults _水位装备class))))
    (Variables|Equipment部分|Set水位装备属性 _returnvalue_3)
    (else
      (GameplayEffects|RemoveActiveGameplayEffect _returnvalue_2 (Variables|Equipment部分|Get水位装备属性) -1))))

(fn DealHuoEquipmentAttributebyClass
  (bind _returnvalue (Components|GetOwner))
  (bind _火位装备class (Variables|Equipment部分|Get火位装备Class))
  (bind _returnvalue_2 (Ability|GetAbilitySystemComponent _returnvalue))
  (if (Utilities|IsValidClass _火位装备class)
    (bind _returnvalue_3 (GameplayEffects|ApplyGameplayEffectToSelf :self _returnvalue_2 :GameplayEffectClass (.属性效果组 (Utilities|GetClassDefaults _火位装备class))))
    (Variables|Equipment部分|Set火位装备属性 _returnvalue_3)
    (else
      (GameplayEffects|RemoveActiveGameplayEffect _returnvalue_2 (Variables|Equipment部分|Get火位装备属性) -1))))

(fn DealTuEquipmentAttributebyClass
  (bind _returnvalue (Components|GetOwner))
  (bind _土位装备class (Variables|Equipment部分|Get土位装备Class))
  (bind _returnvalue_2 (Ability|GetAbilitySystemComponent _returnvalue))
  (if (Utilities|IsValidClass _土位装备class)
    (bind _returnvalue_3 (GameplayEffects|ApplyGameplayEffectToSelf :self _returnvalue_2 :GameplayEffectClass (.属性效果组 (Utilities|GetClassDefaults _土位装备class))))
    (Variables|Equipment部分|Set土位装备属性 _returnvalue_3)
    (else
      (GameplayEffects|RemoveActiveGameplayEffect _returnvalue_2 (Variables|Equipment部分|Get土位装备属性) -1))))

(fn DealMuEquipmentAbilitybyClass
  (bind _木位装备class (Variables|Equipment部分|Get木位装备Class))
  (if (Utilities|IsValidClass _木位装备class)
    (for _array_element (.技能能力组 (Utilities|GetClassDefaults _木位装备class))
      (bind _returnvalue (GameplayAbilities|GiveAbility (Ability|GetAbilitySystemComponent (Components|GetOwner)) _array_element 0 -1))
      (Utilities|Array|Add (Variables|Equipment部分|Get木位装备技能) _returnvalue)
      (Class|AbilitySystemComponent|TryActivateAbility (Ability|GetAbilitySystemComponent (Components|GetOwner)) _returnvalue true))
    (else
      (for _array_element_2 (Variables|Equipment部分|Get木位装备技能)
        (GameplayAbilities|ClearAbility (Ability|GetAbilitySystemComponent (Components|GetOwner)) _array_element_2)
        (Utilities|Array|Clear (Variables|Equipment部分|Get木位装备技能))))))

(fn DealShuiEquipmentAbilitybyClass
  (bind _水位装备class (Variables|Equipment部分|Get水位装备Class))
  (if (Utilities|IsValidClass _水位装备class)
    (for _array_element (.技能能力组 (Utilities|GetClassDefaults _水位装备class))
      (bind _returnvalue (GameplayAbilities|GiveAbility (Ability|GetAbilitySystemComponent (Components|GetOwner)) _array_element 0 -1))
      (Utilities|Array|Add (Variables|Equipment部分|Get水位装备技能) _returnvalue)
      (Class|AbilitySystemComponent|TryActivateAbility (Ability|GetAbilitySystemComponent (Components|GetOwner)) _returnvalue true))
    (else
      (for _array_element_2 (Variables|Equipment部分|Get水位装备技能)
        (GameplayAbilities|ClearAbility (Ability|GetAbilitySystemComponent (Components|GetOwner)) _array_element_2)
        (Utilities|Array|Clear (Variables|Equipment部分|Get水位装备技能))))))

(fn DealHuoEquipmentAbilitybyClass
  (bind _火位装备class (Variables|Equipment部分|Get火位装备Class))
  (if (Utilities|IsValidClass _火位装备class)
    (for _array_element (.技能能力组 (Utilities|GetClassDefaults _火位装备class))
      (bind _returnvalue (GameplayAbilities|GiveAbility (Ability|GetAbilitySystemComponent (Components|GetOwner)) _array_element 0 -1))
      (Utilities|Array|Add (Variables|Equipment部分|Get火位装备技能) _returnvalue)
      (Class|AbilitySystemComponent|TryActivateAbility (Ability|GetAbilitySystemComponent (Components|GetOwner)) _returnvalue true))
    (else
      (for _array_element_2 (Variables|Equipment部分|Get火位装备技能)
        (GameplayAbilities|ClearAbility (Ability|GetAbilitySystemComponent (Components|GetOwner)) _array_element_2)
        (Utilities|Array|Clear (Variables|Equipment部分|Get火位装备技能))))))

(fn DealTuEquipmentAbilitybyClass
  (bind _土位装备class (Variables|Equipment部分|Get土位装备Class))
  (if (Utilities|IsValidClass _土位装备class)
    (for _array_element (.技能能力组 (Utilities|GetClassDefaults _土位装备class))
      (bind _returnvalue (GameplayAbilities|GiveAbility (Ability|GetAbilitySystemComponent (Components|GetOwner)) _array_element 0 -1))
      (Utilities|Array|Add (Variables|Equipment部分|Get土位装备技能) _returnvalue)
      (Class|AbilitySystemComponent|TryActivateAbility (Ability|GetAbilitySystemComponent (Components|GetOwner)) _returnvalue true))
    (else
      (for _array_element_2 (Variables|Equipment部分|Get土位装备技能)
        (GameplayAbilities|ClearAbility (Ability|GetAbilitySystemComponent (Components|GetOwner)) _array_element_2)
        (Utilities|Array|Clear (Variables|Equipment部分|Get土位装备技能))))))

(fn GetCarriedResources
  (return (Variables|Default|GetCarriedResource)))

(event Custom|OnJinEquipmentUpdate_Event
  (DealAbility|DealJinEquipmentAbilitybyClass)
  (DealAttribute|DealJinEquipmentAttributebyClass))

(event Custom|OnMuEquipmentUpdate_Event
  (DealAbility|DealMuEquipmentAbilitybyClass)
  (DealAttribute|DealMuEquipmentAttributebyClass))

(event Custom|OnShuiEquipmentUpdate_Event
  (DealAbility|DealShuiEquipmentAbilitybyClass)
  (DealAttribute|DealShuiEquipmentAttributebyClass))

(event Custom|OnHuoEquipmentUpdate_Event
  (DealAbility|DealHuoEquipmentAbilitybyClass)
  (DealAttribute|DealHuoEquipmentAttributebyClass))

(event Custom|OnTuEquipmentUpdate_Event
  (DealAbility|DealTuEquipmentAbilitybyClass)
  (DealAttribute|DealTuEquipmentAttributebyClass))

(event Custom|OnWeaponEquipmentUpdate_Event
  (DealAttribute|DealWeaponEquipmentAttributebyClass)
  (DealAbility|DealWeaponEquipmentAbilitybyClass))