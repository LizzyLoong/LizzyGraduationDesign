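; GA_BaseAbility is a base Gameplay Ability that provides shared dash and pawn pass-through helpers, with empty activate and end events.
; Dash and AirDash push the owning BP_BaseCharacter along its movement direction with a mass-dependent impulse; Dash scales distance by a large constant, AirDash uses it raw.
; 是否穿透Pawn switches the capsule's Pawn response between Overlap and Block, always on player 0 rather than the ability owner.
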(event Custom|Dash
  (params (距离 :type Integer))
  (bind _asbp_base_character (Utilities|Casting|CastToBP_BaseCharacter (.OwnerActor (Utilities|Struct|BreakGameplayAbilityActorInfo (Ability|GetActorInfo)))))
  (Physics|AddImpulse (Variables|/Script/Engine.Character|GetCharacterMovement _asbp_base_character) (* (Default|获取运动方向 _asbp_base_character) (* 距离 200000)) false))

(event Custom|AirDash
  (params (距离 :type Integer))
  (bind _asbp_base_character (Utilities|Casting|CastToBP_BaseCharacter (.OwnerActor (Utilities|Struct|BreakGameplayAbilityActorInfo (Ability|GetActorInfo)))))
  (Physics|AddImpulse (Variables|/Script/Engine.Character|GetCharacterMovement _asbp_base_character) (* (Default|获取运动方向 _asbp_base_character) 距离) false))

(event Ability|EventActivateAbility)

(event Ability|EventOnEndAbility
  (params (bWasCancelled :type Boolean)))

(fn 是否穿透Pawn
  (params (是 :type Boolean))
  (bind _returnvalue (Game|GetPlayerCharacter 0))
  (bind _capsulecomponent (Variables|/Script/Engine.Character|GetCapsuleComponent _returnvalue))
  (if 是
    (Collision|SetCollisionResponsetoChannel _capsulecomponent "ECC_Pawn" "ECR_Overlap")
    (else
      (Collision|SetCollisionResponsetoChannel _capsulecomponent "ECC_Pawn" "ECR_Block"))))